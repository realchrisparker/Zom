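; BP_Zombie is a zombie actor that assembles a randomized appearance in its construction script, with no gameplay logic in its event graph.
; BuildZombie uses ZombieType (Walker, Runner, Tank, Bloater) to pick body and fitting clothing, while shoes and headwear are type-independent.
; Shoes, pants, shirt and jacket follow the body mesh through leader pose; the head piece is excluded.
; Only Walker gets an anim class assigned, and Tank gets no jacket.
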(fn `BuildZombie`
  (`|ExecutionSequence`
    (:`then_0`
      ;[1 1 1 0.5] Setup Body
      (`self.SetZombieBodySKM`)
      ;[1 1 1 0.5] Setup Anim BP
      (`self.SetZombieAnimBP`))
    (:`then_1`
      ;[1 1 1 0.5] Set Shoes
      (`self.SetShoesSKM`)
      ;[1 1 1 0.5] Set Pants
      (`self.SetPantsSKM`)
      ;[1 1 1 0.5] Set Shirt
      (`self.SetShirtSKM`)
      ;[1 1 1 0.5] Set Jacket
      (`self.SetJacketSKM`)
      ;[1 1 1 0.5] Set Head
      (`self.SetHeadSKM`))
    (:`then_2`
      ;[1 1 1 0.5] Set leader pose to mesh so all sub SKM's act as one with the parent Mesh
      (`SkinnedMeshComponent.SetLeaderPoseComponent` (`self.SKM_Shoes`) (`self.Mesh`) false false)
      (`SkinnedMeshComponent.SetLeaderPoseComponent` (`self.SKM_Pants`) (`self.Mesh`) false false)
      (`SkinnedMeshComponent.SetLeaderPoseComponent` (`self.SKM_Shirt`) (`self.Mesh`) false false)
      (`SkinnedMeshComponent.SetLeaderPoseComponent` (`self.SKM_Jacket`) (`self.Mesh`) false false))))

(fn `SetHeadSKM`
  (bind _skm_head (`self.SKM_Head`))
  (bind _skm_head_2 (`self.SKM_Head`))
  (bind _skm_head_3 (`self.SKM_Head`))
  (switch `int` (`KismetMathLibrary.RandomInteger` 4)
    (:`1`
      ;[1 1 1 0.5] Ball Cap
      (switch `int` (`KismetMathLibrary.RandomInteger` 2)
        (:`0`
          (`SkeletalMeshComponent.SetSkeletalMeshAsset` _skm_head_3 "/Game/ZombieMegaBundle/Mesh_UE5/UE5_Skeleton/Head_Detals/SKM_Cap_Red_UE5.SKM_Cap_Red_UE5"))
        (:`1`
          (`SkeletalMeshComponent.SetSkeletalMeshAsset` _skm_head_3 "/Game/ZombieMegaBundle/Mesh_UE5/UE5_Skeleton/Head_Detals/SKM_Cap_UE5.SKM_Cap_UE5"))
        (:`2`
          (`SkeletalMeshComponent.SetSkeletalMeshAsset` _skm_head_3 "/Game/ZombieMegaBundle/Mesh_UE5/UE5_Skeleton/Head_Detals/SKM_Construction_Helmet_UE5.SKM_Construction_Helmet_UE5"))))
    (:`2`
      ;[1 1 1 0.5] Hair
      (switch `int` (`KismetMathLibrary.RandomInteger` 3)
        (:`0`
          (`SkeletalMeshComponent.SetSkeletalMeshAsset` _skm_head "/Game/ZombieMegaBundle/Mesh_UE5/UE5_Skeleton/Head_Detals/SKM_Hair_Back_Long_UE5.SKM_Hair_Back_Long_UE5"))
        (:`1`
          (`SkeletalMeshComponent.SetSkeletalMeshAsset` _skm_head "/Game/ZombieMegaBundle/Mesh_UE5/UE5_Skeleton/Head_Detals/SKM_Hair_Back_UE5.SKM_Hair_Back_UE5"))
        (:`2`
          (`SkeletalMeshComponent.SetSkeletalMeshAsset` _skm_head "/Game/ZombieMegaBundle/Mesh_UE5/UE5_Skeleton/Head_Detals/SKM_Hair_Short_UE5.SKM_Hair_Short_UE5"))
        (:`3`
          (`SkeletalMeshComponent.SetSkeletalMeshAsset` _skm_head "/Game/ZombieMegaBundle/Mesh_UE5/UE5_Skeleton/Head_Detals/SKM_Long_Hair_UE5.SKM_Long_Hair_UE5"))))
    (:`3`
      ;[1 1 1 0.5] Skull Cap
      (switch `int` (`KismetMathLibrary.RandomInteger` 2)
        (:`0`
          (`SkeletalMeshComponent.SetSkeletalMeshAsset` _skm_head_2 "/Game/ZombieMegaBundle/Mesh_UE5/UE5_Skeleton/Head_Detals/SKM_Warm_Hat_Black_UE5.SKM_Warm_Hat_Black_UE5"))
        (:`1`
          (`SkeletalMeshComponent.SetSkeletalMeshAsset` _skm_head_2 "/Game/ZombieMegaBundle/Mesh_UE5/UE5_Skeleton/Head_Detals/SKM_Warm_Hat_UE5.SKM_Warm_Hat_UE5"))))))

(fn `SetJacketSKM`
  (bind _skm_jacket (`self.SKM_Jacket`))
  (bind _skm_jacket_2 (`self.SKM_Jacket`))
  (switch `EZombieType` (`self.ZombieType`)
    (:`Walker`
      ;[1 1 1 0.5] Skinny & Normal
      (switch `int` (`KismetMathLibrary.RandomInteger` 6) :!label _label
        (:`0`
          (`SkeletalMeshComponent.SetSkeletalMeshAsset` _skm_jacket_2 "/Game/ZombieMegaBundle/Mesh_UE5/UE5_Skeleton/Cloth_Top/SKM_Jaket_Dark_UE5.SKM_Jaket_Dark_UE5"))
        (:`1`
          (`SkeletalMeshComponent.SetSkeletalMeshAsset` _skm_jacket_2 "/Game/ZombieMegaBundle/Mesh_UE5/UE5_Skeleton/Cloth_Top/SKM_Jaket_Jeans_Blue_UE5.SKM_Jaket_Jeans_Blue_UE5"))
        (:`2`
          (`SkeletalMeshComponent.SetSkeletalMeshAsset` _skm_jacket_2 "/Game/ZombieMegaBundle/Mesh_UE5/UE5_Skeleton/Cloth_Top/SKM_Jaket_Jeans_Gray_UE5.SKM_Jaket_Jeans_Gray_UE5"))
        (:`3`
          (`SkeletalMeshComponent.SetSkeletalMeshAsset` _skm_jacket_2 "/Game/ZombieMegaBundle/Mesh_UE5/UE5_Skeleton/Cloth_Top/SKM_Jaket_Jeans_Red_UE5.SKM_Jaket_Jeans_Red_UE5"))
        (:`4`
          (`SkeletalMeshComponent.SetSkeletalMeshAsset` _skm_jacket_2 "/Game/ZombieMegaBundle/Mesh_UE5/UE5_Skeleton/Cloth_Top/SKM_Jaket_Jeans_UE5.SKM_Jaket_Jeans_UE5"))
        (:`5`
          (`SkeletalMeshComponent.SetSkeletalMeshAsset` _skm_jacket_2 "/Game/ZombieMegaBundle/Mesh_UE5/UE5_Skeleton/Cloth_Top/SKM_Jaket_UE5.SKM_Jaket_UE5"))))
    (:`Runner`
      (goto _label))
    (:`Bloater`
      ;[1 1 1 0.5] Fat (Bloater)
      (switch `int` (`KismetMathLibrary.RandomInteger` 5)
        (:`0`
          (`SkeletalMeshComponent.SetSkeletalMeshAsset` _skm_jacket "/Game/ZombieMegaBundle/Mesh_UE5/UE5_Skeleton/Cloth_Top/Fat/SKM_Fat_Jaket_Blue_UE5.SKM_Fat_Jaket_Blue_UE5"))
        (:`1`
          (`SkeletalMeshComponent.SetSkeletalMeshAsset` _skm_jacket "/Game/ZombieMegaBundle/Mesh_UE5/UE5_Skeleton/Cloth_Top/Fat/SKM_Fat_Jaket_Jeans_Blue_UE5.SKM_Fat_Jaket_Jeans_Blue_UE5"))
        (:`2`
          (`SkeletalMeshComponent.SetSkeletalMeshAsset` _skm_jacket "/Game/ZombieMegaBundle/Mesh_UE5/UE5_Skeleton/Cloth_Top/Fat/SKM_Fat_Jaket_Jeans_Gray_UE5.SKM_Fat_Jaket_Jeans_Gray_UE5"))
        (:`3`
          (`SkeletalMeshComponent.SetSkeletalMeshAsset` _skm_jacket "/Game/ZombieMegaBundle/Mesh_UE5/UE5_Skeleton/Cloth_Top/Fat/SKM_Fat_Jaket_Jeans_Red_UE5.SKM_Fat_Jaket_Jeans_Red_UE5"))
        (:`4`
          (`SkeletalMeshComponent.SetSkeletalMeshAsset` _skm_jacket "/Game/ZombieMegaBundle/Mesh_UE5/UE5_Skeleton/Cloth_Top/Fat/SKM_Fat_Jaket_Jeans_UE5.SKM_Fat_Jaket_Jeans_UE5"))))))

(fn `SetPantsSKM`
  (bind _skm_pants (`self.SKM_Pants`))
  (bind _skm_pants_2 (`self.SKM_Pants`))
  (bind _skm_pants_3 (`self.SKM_Pants`))
  (switch `EZombieType` (`self.ZombieType`)
    (:`Walker`
      ;[1 1 1 0.5] Skinny & Normal
      (switch `int` (`KismetMathLibrary.RandomInteger` 16) :!label _label
        (:`0`
          (`SkeletalMeshComponent.SetSkeletalMeshAsset` _skm_pants_3 "/Game/ZombieMegaBundle/Mesh_UE5/UE5_Skeleton/Pants/SKM_Jeans_Half_Blue_UE5.SKM_Jeans_Half_Blue_UE5"))
        (:`1`
          (`SkeletalMeshComponent.SetSkeletalMeshAsset` _skm_pants_3 "/Game/ZombieMegaBundle/Mesh_UE5/UE5_Skeleton/Pants/SKM_Jeans_Half_Gray_UE5.SKM_Jeans_Half_Gray_UE5"))
        (:`2`
          (`SkeletalMeshComponent.SetSkeletalMeshAsset` _skm_pants_3 "/Game/ZombieMegaBundle/Mesh_UE5/UE5_Skeleton/Pants/SKM_Jeans_Half_UE5.SKM_Jeans_Half_UE5"))
        (:`3`
          (`SkeletalMeshComponent.SetSkeletalMeshAsset` _skm_pants_3 "/Game/ZombieMegaBundle/Mesh_UE5/UE5_Skeleton/Pants/SKM_Jeans_Long_Blue_UE5.SKM_Jeans_Long_Blue_UE5"))
        (:`4`
          (`SkeletalMeshComponent.SetSkeletalMeshAsset` _skm_pants_3 "/Game/ZombieMegaBundle/Mesh_UE5/UE5_Skeleton/Pants/SKM_Jeans_Long_Gray_UE5.SKM_Jeans_Long_Gray_UE5"))
        (:`5`
          (`SkeletalMeshComponent.SetSkeletalMeshAsset` _skm_pants_3 "/Game/ZombieMegaBundle/Mesh_UE5/UE5_Skeleton/Pants/SKM_Jeans_Long_UE5.SKM_Jeans_Long_UE5"))
        (:`6`
          (`SkeletalMeshComponent.SetSkeletalMeshAsset` _skm_pants_3 "/Game/ZombieMegaBundle/Mesh_UE5/UE5_Skeleton/Pants/SKM_Jeans_Shorts_Blue_UE5.SKM_Jeans_Shorts_Blue_UE5"))
        (:`7`
          (`SkeletalMeshComponent.SetSkeletalMeshAsset` _skm_pants_3 "/Game/ZombieMegaBundle/Mesh_UE5/UE5_Skeleton/Pants/SKM_Jeans_Shorts_Gray_UE5.SKM_Jeans_Shorts_Gray_UE5"))
        (:`8`
          (`SkeletalMeshComponent.SetSkeletalMeshAsset` _skm_pants_3 "/Game/ZombieMegaBundle/Mesh_UE5/UE5_Skeleton/Pants/SKM_Jeans_Shorts_UE5.SKM_Jeans_Shorts_UE5"))
        (:`9`
          (`SkeletalMeshComponent.SetSkeletalMeshAsset` _skm_pants_3 "/Game/ZombieMegaBundle/Mesh_UE5/UE5_Skeleton/Pants/SKM_Pants_Half_Brown_UE5.SKM_Pants_Half_Brown_UE5"))
        (:`10`
          (`SkeletalMeshComponent.SetSkeletalMeshAsset` _skm_pants_3 "/Game/ZombieMegaBundle/Mesh_UE5/UE5_Skeleton/Pants/SKM_Pants_Half_Gray_UE5.SKM_Pants_Half_Gray_UE5"))
        (:`11`
          (`SkeletalMeshComponent.SetSkeletalMeshAsset` _skm_pants_3 "/Game/ZombieMegaBundle/Mesh_UE5/UE5_Skeleton/Pants/SKM_Pants_Half_UE5.SKM_Pants_Half_UE5"))
        (:`12`
          (`SkeletalMeshComponent.SetSkeletalMeshAsset` _skm_pants_3 "/Game/ZombieMegaBundle/Mesh_UE5/UE5_Skeleton/Pants/SKM_Pants_Long_Brown_UE5.SKM_Pants_Long_Brown_UE5"))
        (:`13`
          (`SkeletalMeshComponent.SetSkeletalMeshAsset` _skm_pants_3 "/Game/ZombieMegaBundle/Mesh_UE5/UE5_Skeleton/Pants/SKM_Pants_Long_Gray_UE5.SKM_Pants_Long_Gray_UE5"))
        (:`14`
          (`SkeletalMeshComponent.SetSkeletalMeshAsset` _skm_pants_3 "/Game/ZombieMegaBundle/Mesh_UE5/UE5_Skeleton/Pants/SKM_Pants_Long_UE5.SKM_Pants_Long_UE5"))
        (:`15`
          (`SkeletalMeshComponent.SetSkeletalMeshAsset` _skm_pants_3 "/Game/ZombieMegaBundle/Mesh_UE5/UE5_Skeleton/Pants/SKM_Pants_Short_Brown_UE5.SKM_Pants_Short_Brown_UE5"))
        (:`16`
          (`SkeletalMeshComponent.SetSkeletalMeshAsset` _skm_pants_3 "/Game/ZombieMegaBundle/Mesh_UE5/UE5_Skeleton/Pants/SKM_Pants_Short_Gray_UE5.SKM_Pants_Short_Gray_UE5"))
        (:`17`
          (`SkeletalMeshComponent.SetSkeletalMeshAsset` _skm_pants_3 "/Game/ZombieMegaBundle/Mesh_UE5/UE5_Skeleton/Pants/SKM_Pants_Short_UE5.SKM_Pants_Short_UE5"))))
    (:`Runner`
      (goto _label))
    (:`Tank`
      ;[1 1 1 0.5] Muscle (Tank)
      (switch `int` (`KismetMathLibrary.RandomInteger` 8)
        (:`0`
          (`SkeletalMeshComponent.SetSkeletalMeshAsset` _skm_pants "/Game/ZombieMegaBundle/Mesh_UE5/UE5_Skeleton/Pants/Muscle/SKM_Jeans_Long_Muscle_Blue_UE5.SKM_Jeans_Long_Muscle_Blue_UE5"))
        (:`1`
          (`SkeletalMeshComponent.SetSkeletalMeshAsset` _skm_pants "/Game/ZombieMegaBundle/Mesh_UE5/UE5_Skeleton/Pants/Muscle/SKM_Jeans_Long_Muscle_Gray_UE5.SKM_Jeans_Long_Muscle_Gray_UE5"))
        (:`2`
          (`SkeletalMeshComponent.SetSkeletalMeshAsset` _skm_pants "/Game/ZombieMegaBundle/Mesh_UE5/UE5_Skeleton/Pants/Muscle/SKM_Jeans_Long_Muscle_UE5.SKM_Jeans_Long_Muscle_UE5"))
        (:`3`
          (`SkeletalMeshComponent.SetSkeletalMeshAsset` _skm_pants "/Game/ZombieMegaBundle/Mesh_UE5/UE5_Skeleton/Pants/Muscle/SKM_Jeans_Shorts_Muscle_Blue_UE5.SKM_Jeans_Shorts_Muscle_Blue_UE5"))
        (:`4`
          (`SkeletalMeshComponent.SetSkeletalMeshAsset` _skm_pants "/Game/ZombieMegaBundle/Mesh_UE5/UE5_Skeleton/Pants/Muscle/SKM_Jeans_Shorts_Muscle_Gray_UE5.SKM_Jeans_Shorts_Muscle_Gray_UE5"))
        (:`5`
          (`SkeletalMeshComponent.SetSkeletalMeshAsset` _skm_pants "/Game/ZombieMegaBundle/Mesh_UE5/UE5_Skeleton/Pants/Muscle/SKM_Jeans_Shorts_Muscle_UE5.SKM_Jeans_Shorts_Muscle_UE5"))
        (:`6`
          (`SkeletalMeshComponent.SetSkeletalMeshAsset` _skm_pants "/Game/ZombieMegaBundle/Mesh_UE5/UE5_Skeleton/Pants/Muscle/SKM_Pants_Short_Muscle_Brown_UE5.SKM_Pants_Short_Muscle_Brown_UE5"))
        (:`7`
          (`SkeletalMeshComponent.SetSkeletalMeshAsset` _skm_pants "/Game/ZombieMegaBundle/Mesh_UE5/UE5_Skeleton/Pants/Muscle/SKM_Pants_Short_Muscle_Gray_UE5.SKM_Pants_Short_Muscle_Gray_UE5"))
        (:`8`
          (`SkeletalMeshComponent.SetSkeletalMeshAsset` _skm_pants "/Game/ZombieMegaBundle/Mesh_UE5/UE5_Skeleton/Pants/Muscle/SKM_Pants_Short_Muscle_UE5.SKM_Pants_Short_Muscle_UE5"))))
    (:`Bloater`
      ;[1 1 1 0.5] Fat (Bloater)
      (switch `int` (`KismetMathLibrary.RandomInteger` 5)
        (:`0`
          (`SkeletalMeshComponent.SetSkeletalMeshAsset` _skm_pants_2 "/Game/ZombieMegaBundle/Mesh_UE5/UE5_Skeleton/Pants/Fat/SKM_Fat_Jeans_Half_Blue_UE5.SKM_Fat_Jeans_Half_Blue_UE5"))
        (:`1`
          (`SkeletalMeshComponent.SetSkeletalMeshAsset` _skm_pants_2 "/Game/ZombieMegaBundle/Mesh_UE5/UE5_Skeleton/Pants/Fat/SKM_Fat_Jeans_Half_Gray_UE5.SKM_Fat_Jeans_Half_Gray_UE5"))
        (:`2`
          (`SkeletalMeshComponent.SetSkeletalMeshAsset` _skm_pants_2 "/Game/ZombieMegaBundle/Mesh_UE5/UE5_Skeleton/Pants/Fat/SKM_Fat_Jeans_Half_UE5.SKM_Fat_Jeans_Half_UE5"))
        (:`3`
          (`SkeletalMeshComponent.SetSkeletalMeshAsset` _skm_pants_2 "/Game/ZombieMegaBundle/Mesh_UE5/UE5_Skeleton/Pants/Fat/SKM_Fat_Jeans_Shorts_Blue_UE5.SKM_Fat_Jeans_Shorts_Blue_UE5"))
        (:`4`
          (`SkeletalMeshComponent.SetSkeletalMeshAsset` _skm_pants_2 "/Game/ZombieMegaBundle/Mesh_UE5/UE5_Skeleton/Pants/Fat/SKM_Fat_Jeans_Shorts_Gray_UE5.SKM_Fat_Jeans_Shorts_Gray_UE5"))
        (:`5`
          (`SkeletalMeshComponent.SetSkeletalMeshAsset` _skm_pants_2 "/Game/ZombieMegaBundle/Mesh_UE5/UE5_Skeleton/Pants/Fat/SKM_Fat_Jeans_Shorts_UE5.SKM_Fat_Jeans_Shorts_UE5"))))))

(fn `SetShirtSKM`
  (bind _skm_shirt (`self.SKM_Shirt`))
  (bind _skm_shirt_2 (`self.SKM_Shirt`))
  (bind _skm_shirt_3 (`self.SKM_Shirt`))
  (bind _skm_shirt_4 (`self.SKM_Shirt`))
  (bind _skm_shirt_5 (`self.SKM_Shirt`))
  (bind _skm_shirt_6 (`self.SKM_Shirt`))
  (bind _skm_shirt_7 (`self.SKM_Shirt`))
  (bind _skm_shirt_8 (`self.SKM_Shirt`))
  (bind _skm_shirt_9 (`self.SKM_Shirt`))
  (bind _skm_shirt_10 (`self.SKM_Shirt`))
  (switch `EZombieType` (`self.ZombieType`)
    (:`Walker`
      ;[1 1 1 0.5] Skinny & Normal
      (switch `int` (`KismetMathLibrary.RandomInteger` 4) :!label _label
        (:`1`
          ;;[1 1 1 0.5] Long Sleeve Shirt
          (switch `int` (`KismetMathLibrary.RandomInteger` 9)
            (:`0`
              (`SkeletalMeshComponent.SetSkeletalMeshAsset` _skm_shirt_6 "/Game/ZombieMegaBundle/Mesh_UE5/UE5_Skeleton/Cloth/Shirt/SKM_Shirt_Black_Blood_UE5.SKM_Shirt_Black_Blood_UE5"))
            (:`1`
              (`SkeletalMeshComponent.SetSkeletalMeshAsset` _skm_shirt_6 "/Game/ZombieMegaBundle/Mesh_UE5/UE5_Skeleton/Cloth/Shirt/SKM_Shirt_Black_UE5.SKM_Shirt_Black_UE5"))
            (:`2`
              (`SkeletalMeshComponent.SetSkeletalMeshAsset` _skm_shirt_6 "/Game/ZombieMegaBundle/Mesh_UE5/UE5_Skeleton/Cloth/Shirt/SKM_Shirt_Blood_UE5.SKM_Shirt_Blood_UE5"))
            (:`3`
              (`SkeletalMeshComponent.SetSkeletalMeshAsset` _skm_shirt_6 "/Game/ZombieMegaBundle/Mesh_UE5/UE5_Skeleton/Cloth/Shirt/SKM_Shirt_Blue_Blood_UE5.SKM_Shirt_Blue_Blood_UE5"))
            (:`4`
              (`SkeletalMeshComponent.SetSkeletalMeshAsset` _skm_shirt_6 "/Game/ZombieMegaBundle/Mesh_UE5/UE5_Skeleton/Cloth/Shirt/SKM_Shirt_Hawaii_Blue_UE5.SKM_Shirt_Hawaii_Blue_UE5"))
            (:`5`
              (`SkeletalMeshComponent.SetSkeletalMeshAsset` _skm_shirt_6 "/Game/ZombieMegaBundle/Mesh_UE5/UE5_Skeleton/Cloth/Shirt/SKM_Shirt_Hawaii_Red_UE5.SKM_Shirt_Hawaii_Red_UE5"))
            (:`6`
              (`SkeletalMeshComponent.SetSkeletalMeshAsset` _skm_shirt_6 "/Game/ZombieMegaBundle/Mesh_UE5/UE5_Skeleton/Cloth/Shirt/SKM_Shirt_UE5.SKM_Shirt_UE5"))
            (:`7`
              (`SkeletalMeshComponent.SetSkeletalMeshAsset` _skm_shirt_6 "/Game/ZombieMegaBundle/Mesh_UE5/UE5_Skeleton/Cloth/Shirt/SKM_Shirt_White_Blood_UE5.SKM_Shirt_White_Blood_UE5"))
            (:`8`
              (`SkeletalMeshComponent.SetSkeletalMeshAsset` _skm_shirt_6 "/Game/ZombieMegaBundle/Mesh_UE5/UE5_Skeleton/Cloth/Shirt/SKM_Shirt_Blue_UE5.SKM_Shirt_Blue_UE5"))
            (:`9`
              (`SkeletalMeshComponent.SetSkeletalMeshAsset` _skm_shirt_6 "/Game/ZombieMegaBundle/Mesh_UE5/UE5_Skeleton/Cloth/Shirt/SKM_Shirt_White_UE5.SKM_Shirt_White_UE5"))))
        (:`2`
          ;;[1 1 1 0.5] Sleeveless T-Shirt
          (switch `int` (`KismetMathLibrary.RandomInteger` 3)
            (:`0`
              (`SkeletalMeshComponent.SetSkeletalMeshAsset` _skm_shirt_8 "/Game/ZombieMegaBundle/Mesh_UE5/UE5_Skeleton/Cloth/Sleeveless_Tshirt/SKM_Sleeveless_Tshirt_Blood_UE5.SKM_Sleeveless_Tshirt_Blood_UE5"))
            (:`1`
              (`SkeletalMeshComponent.SetSkeletalMeshAsset` _skm_shirt_8 "/Game/ZombieMegaBundle/Mesh_UE5/UE5_Skeleton/Cloth/Sleeveless_Tshirt/SKM_Sleeveless_Tshirt_UE5.SKM_Sleeveless_Tshirt_UE5"))
            (:`2`
              (`SkeletalMeshComponent.SetSkeletalMeshAsset` _skm_shirt_8 "/Game/ZombieMegaBundle/Mesh_UE5/UE5_Skeleton/Cloth/Sleeveless_Tshirt/SKM_Sleeveless_Tshirt_White_Blood_UE5.SKM_Sleeveless_Tshirt_White_Blood_UE5"))
            (:`3`
              (`SkeletalMeshComponent.SetSkeletalMeshAsset` _skm_shirt_8 "/Game/ZombieMegaBundle/Mesh_UE5/UE5_Skeleton/Cloth/Sleeveless_Tshirt/SKM_Sleeveless_Tshirt_White_UE5.SKM_Sleeveless_Tshirt_White_UE5"))))
        (:`3`
          ;;[1 1 1 0.5] T-Shirt Damaged
          (switch `int` (`KismetMathLibrary.RandomInteger` 9)
            (:`0`
              (`SkeletalMeshComponent.SetSkeletalMeshAsset` _skm_shirt_9 "/Game/ZombieMegaBundle/Mesh_UE5/UE5_Skeleton/Cloth/Tshirt/SKM_Tshirt_Black_Blood_UE5.SKM_Tshirt_Black_Blood_UE5"))
            (:`1`
              (`SkeletalMeshComponent.SetSkeletalMeshAsset` _skm_shirt_9 "/Game/ZombieMegaBundle/Mesh_UE5/UE5_Skeleton/Cloth/Tshirt/SKM_Tshirt_Black_Logo_UE5.SKM_Tshirt_Black_Logo_UE5"))
            (:`2`
              (`SkeletalMeshComponent.SetSkeletalMeshAsset` _skm_shirt_9 "/Game/ZombieMegaBundle/Mesh_UE5/UE5_Skeleton/Cloth/Tshirt/SKM_Tshirt_Black_UE5.SKM_Tshirt_Black_UE5"))
            (:`3`
              (`SkeletalMeshComponent.SetSkeletalMeshAsset` _skm_shirt_9 "/Game/ZombieMegaBundle/Mesh_UE5/UE5_Skeleton/Cloth/Tshirt/SKM_Tshirt_Blood_UE5.SKM_Tshirt_Blood_UE5"))
            (:`4`
              (`SkeletalMeshComponent.SetSkeletalMeshAsset` _skm_shirt_9 "/Game/ZombieMegaBundle/Mesh_UE5/UE5_Skeleton/Cloth/Tshirt/SKM_Tshirt_Blue_UE5.SKM_Tshirt_Blue_UE5"))
            (:`5`
              (`SkeletalMeshComponent.SetSkeletalMeshAsset` _skm_shirt_9 "/Game/ZombieMegaBundle/Mesh_UE5/UE5_Skeleton/Cloth/Tshirt/SKM_Tshirt_Green_Blood_UE5.SKM_Tshirt_Green_Blood_UE5"))
            (:`6`
              (`SkeletalMeshComponent.SetSkeletalMeshAsset` _skm_shirt_9 "/Game/ZombieMegaBundle/Mesh_UE5/UE5_Skeleton/Cloth/Tshirt/SKM_Tshirt_Green_UE5.SKM_Tshirt_Green_UE5"))
            (:`7`
              (`SkeletalMeshComponent.SetSkeletalMeshAsset` _skm_shirt_9 "/Game/ZombieMegaBundle/Mesh_UE5/UE5_Skeleton/Cloth/Tshirt/SKM_Tshirt_UE5.SKM_Tshirt_UE5"))
            (:`8`
              (`SkeletalMeshComponent.SetSkeletalMeshAsset` _skm_shirt_9 "/Game/ZombieMegaBundle/Mesh_UE5/UE5_Skeleton/Cloth/Tshirt/SKM_Tshirt_Blue_Blood_UE5.SKM_Tshirt_Blue_Blood_UE5"))
            (:`9`
              (`SkeletalMeshComponent.SetSkeletalMeshAsset` _skm_shirt_9 "/Game/ZombieMegaBundle/Mesh_UE5/UE5_Skeleton/Cloth/Tshirt/SKM_Tshirt_White_Blood_UE5.SKM_Tshirt_White_Blood_UE5"))
            (:`10`
              (`SkeletalMeshComponent.SetSkeletalMeshAsset` _skm_shirt_9 "/Game/ZombieMegaBundle/Mesh_UE5/UE5_Skeleton/Cloth/Tshirt/SKM_Tshirt_White_UE5.SKM_Tshirt_White_UE5"))))
        (:`4`
          ;;[1 1 1 0.5] T-Shirt
          (switch `int` (`KismetMathLibrary.RandomInteger` 3)
            (:`0`
              (`SkeletalMeshComponent.SetSkeletalMeshAsset` _skm_shirt_2 "/Game/ZombieMegaBundle/Mesh_UE5/UE5_Skeleton/Cloth/Tshirt_Demaged/SKM_TShirt_Demaged_Black_UE5.SKM_TShirt_Demaged_Black_UE5"))
            (:`1`
              (`SkeletalMeshComponent.SetSkeletalMeshAsset` _skm_shirt_2 "/Game/ZombieMegaBundle/Mesh_UE5/UE5_Skeleton/Cloth/Tshirt_Demaged/SKM_TShirt_Demaged_Red_UE5.SKM_TShirt_Demaged_Red_UE5"))
            (:`2`
              (`SkeletalMeshComponent.SetSkeletalMeshAsset` _skm_shirt_2 "/Game/ZombieMegaBundle/Mesh_UE5/UE5_Skeleton/Cloth/Tshirt_Demaged/SKM_TShirt_Demaged_UE5.SKM_TShirt_Demaged_UE5"))
            (:`3`
              (`SkeletalMeshComponent.SetSkeletalMeshAsset` _skm_shirt_2 "/Game/ZombieMegaBundle/Mesh_UE5/UE5_Skeleton/Cloth/Tshirt_Demaged/SKM_TShirt_Demaged_White_UE5.SKM_TShirt_Demaged_White_UE5"))))))
    (:`Runner`
      (goto _label))
    (:`Tank`
      ;[1 1 1 0.5] Muscle (Tank)
      (switch `int` (`KismetMathLibrary.RandomInteger` 3)
        (:`0`
          ;;[1 1 1 0.5] Sleeveless T-Shirt
          (switch `int` (`KismetMathLibrary.RandomInteger` 3)
            (:`0`
              (`SkeletalMeshComponent.SetSkeletalMeshAsset` _skm_shirt_3 "/Game/ZombieMegaBundle/Mesh_UE5/UE5_Skeleton/Cloth/Sleeveless_Tshirt/Muscle/SKM_Muscle_Sleeveless_Tshirt_Blood_UE5.SKM_Muscle_Sleeveless_Tshirt_Blood_UE5"))
            (:`1`
              (`SkeletalMeshComponent.SetSkeletalMeshAsset` _skm_shirt_3 "/Game/ZombieMegaBundle/Mesh_UE5/UE5_Skeleton/Cloth/Sleeveless_Tshirt/Muscle/SKM_Muscle_Sleeveless_Tshirt_UE5.SKM_Muscle_Sleeveless_Tshirt_UE5"))
            (:`2`
              (`SkeletalMeshComponent.SetSkeletalMeshAsset` _skm_shirt_3 "/Game/ZombieMegaBundle/Mesh_UE5/UE5_Skeleton/Cloth/Sleeveless_Tshirt/Muscle/SKM_Muscle_Sleeveless_Tshirt_White_Blood_UE5.SKM_Muscle_Sleeveless_Tshirt_White_Blood_UE5"))
            (:`3`
              (`SkeletalMeshComponent.SetSkeletalMeshAsset` _skm_shirt_3 "/Game/ZombieMegaBundle/Mesh_UE5/UE5_Skeleton/Cloth/Sleeveless_Tshirt/Muscle/SKM_Muscle_Sleeveless_Tshirt_White_UE5.SKM_Muscle_Sleeveless_Tshirt_White_UE5"))))
        (:`1`
          ;;[1 1 1 0.5] T-Shirt
          (switch `int` (`KismetMathLibrary.RandomInteger` 11)
            (:`0`
              (`SkeletalMeshComponent.SetSkeletalMeshAsset` _skm_shirt_4 "/Game/ZombieMegaBundle/Mesh_UE5/UE5_Skeleton/Cloth/Tshirt/Muscle/SKM_Muscle_Tsirt_Black_Blood_UE5.SKM_Muscle_Tsirt_Black_Blood_UE5"))
            (:`1`
              (`SkeletalMeshComponent.SetSkeletalMeshAsset` _skm_shirt_4 "/Game/ZombieMegaBundle/Mesh_UE5/UE5_Skeleton/Cloth/Tshirt/Muscle/SKM_Muscle_Tsirt_Black_UE5.SKM_Muscle_Tsirt_Black_UE5"))
            (:`2`
              (`SkeletalMeshComponent.SetSkeletalMeshAsset` _skm_shirt_4 "/Game/ZombieMegaBundle/Mesh_UE5/UE5_Skeleton/Cloth/Tshirt/Muscle/SKM_Muscle_Tsirt_Blood_UE5.SKM_Muscle_Tsirt_Blood_UE5"))
            (:`3`
              (`SkeletalMeshComponent.SetSkeletalMeshAsset` _skm_shirt_4 "/Game/ZombieMegaBundle/Mesh_UE5/UE5_Skeleton/Cloth/Tshirt/Muscle/SKM_Muscle_Tsirt_Blue_Blood_UE5.SKM_Muscle_Tsirt_Blue_Blood_UE5"))
            (:`4`
              (`SkeletalMeshComponent.SetSkeletalMeshAsset` _skm_shirt_4 "/Game/ZombieMegaBundle/Mesh_UE5/UE5_Skeleton/Cloth/Tshirt/Muscle/SKM_Muscle_Tsirt_Green_UE5.SKM_Muscle_Tsirt_Green_UE5"))
            (:`5`
              (`SkeletalMeshComponent.SetSkeletalMeshAsset` _skm_shirt_4 "/Game/ZombieMegaBundle/Mesh_UE5/UE5_Skeleton/Cloth/Tshirt/Muscle/SKM_Muscle_Tsirt_Logo_Black_UE5.SKM_Muscle_Tsirt_Logo_Black_UE5"))
            (:`6`
              (`SkeletalMeshComponent.SetSkeletalMeshAsset` _skm_shirt_4 "/Game/ZombieMegaBundle/Mesh_UE5/UE5_Skeleton/Cloth/Tshirt/Muscle/SKM_Muscle_Tsirt_Logo_UE5.SKM_Muscle_Tsirt_Logo_UE5"))
            (:`7`
              (`SkeletalMeshComponent.SetSkeletalMeshAsset` _skm_shirt_4 "/Game/ZombieMegaBundle/Mesh_UE5/UE5_Skeleton/Cloth/Tshirt/Muscle/SKM_Muscle_Tsirt_White_Blood_UE5.SKM_Muscle_Tsirt_White_Blood_UE5"))
            (:`8`
              (`SkeletalMeshComponent.SetSkeletalMeshAsset` _skm_shirt_4 "/Game/ZombieMegaBundle/Mesh_UE5/UE5_Skeleton/Cloth/Tshirt/Muscle/SKM_Muscle_Tsirt_Blue_UE5.SKM_Muscle_Tsirt_Blue_UE5"))
            (:`9`
              (`SkeletalMeshComponent.SetSkeletalMeshAsset` _skm_shirt_4 "/Game/ZombieMegaBundle/Mesh_UE5/UE5_Skeleton/Cloth/Tshirt/Muscle/SKM_Muscle_Tsirt_White_UE5.SKM_Muscle_Tsirt_White_UE5"))
            (:`10`
              (`SkeletalMeshComponent.SetSkeletalMeshAsset` _skm_shirt_4 "/Game/ZombieMegaBundle/Mesh_UE5/UE5_Skeleton/Cloth/Tshirt/Muscle/SKM_Muscle_Tsirt_Green_Blood_UE5.SKM_Muscle_Tsirt_Green_Blood_UE5"))))
        (:`2`
          ;;[1 1 1 0.5] T-Shirt Damaged
          (switch `int` (`KismetMathLibrary.RandomInteger` 3)
            (:`0`
              (`SkeletalMeshComponent.SetSkeletalMeshAsset` _skm_shirt_5 "/Game/ZombieMegaBundle/Mesh_UE5/UE5_Skeleton/Cloth/Tshirt_Demaged/Muscle/SKM_Muscle_TShirt_Demaged_Black_UE5.SKM_Muscle_TShirt_Demaged_Black_UE5"))
            (:`1`
              (`SkeletalMeshComponent.SetSkeletalMeshAsset` _skm_shirt_5 "/Game/ZombieMegaBundle/Mesh_UE5/UE5_Skeleton/Cloth/Tshirt_Demaged/Muscle/SKM_Muscle_TShirt_Demaged_Red_UE5.SKM_Muscle_TShirt_Demaged_Red_UE5"))
            (:`2`
              (`SkeletalMeshComponent.SetSkeletalMeshAsset` _skm_shirt_5 "/Game/ZombieMegaBundle/Mesh_UE5/UE5_Skeleton/Cloth/Tshirt_Demaged/Muscle/SKM_Muscle_TShirt_Demaged_UE5.SKM_Muscle_TShirt_Demaged_UE5"))
            (:`3`
              (`SkeletalMeshComponent.SetSkeletalMeshAsset` _skm_shirt_5 "/Game/ZombieMegaBundle/Mesh_UE5/UE5_Skeleton/Cloth/Tshirt_Demaged/Muscle/SKM_Muscle_TShirt_Demaged_White_UE5.SKM_Muscle_TShirt_Demaged_White_UE5"))))))
    (:`Bloater`
      ;[1 1 1 0.5] Fat (Bloater)
      (switch `int` (`KismetMathLibrary.RandomInteger` 3)
        (:`0`
          ;;[1 1 1 0.5] Sleeveless T-Shirt
          (switch `int` (`KismetMathLibrary.RandomInteger` 6)
            (:`0`
              (`SkeletalMeshComponent.SetSkeletalMeshAsset` _skm_shirt_10 "/Game/ZombieMegaBundle/Mesh_UE5/UE5_Skeleton/Cloth/Sleeveless_Tshirt/Fat/SKM_Fat_Sleeveless_Tshirt_Blood_UE5.SKM_Fat_Sleeveless_Tshirt_Blood_UE5"))
            (:`1`
              (`SkeletalMeshComponent.SetSkeletalMeshAsset` _skm_shirt_10 "/Game/ZombieMegaBundle/Mesh_UE5/UE5_Skeleton/Cloth/Sleeveless_Tshirt/Fat/SKM_Fat_Sleeveless_Tshirt_Gray_Blood_UE5.SKM_Fat_Sleeveless_Tshirt_Gray_Blood_UE5"))
            (:`2`
              (`SkeletalMeshComponent.SetSkeletalMeshAsset` _skm_shirt_10 "/Game/ZombieMegaBundle/Mesh_UE5/UE5_Skeleton/Cloth/Sleeveless_Tshirt/Fat/SKM_Fat_Sleeveless_Tshirt_Gray_UE5.SKM_Fat_Sleeveless_Tshirt_Gray_UE5"))
            (:`3`
              (`SkeletalMeshComponent.SetSkeletalMeshAsset` _skm_shirt_10 "/Game/ZombieMegaBundle/Mesh_UE5/UE5_Skeleton/Cloth/Sleeveless_Tshirt/Fat/SKM_Fat_Sleeveless_Tshirt_Orange_Blood_UE5.SKM_Fat_Sleeveless_Tshirt_Orange_Blood_UE5"))
            (:`4`
              (`SkeletalMeshComponent.SetSkeletalMeshAsset` _skm_shirt_10 "/Game/ZombieMegaBundle/Mesh_UE5/UE5_Skeleton/Cloth/Sleeveless_Tshirt/Fat/SKM_Fat_Sleeveless_Tshirt_Orange_UE5.SKM_Fat_Sleeveless_Tshirt_Orange_UE5"))
            (:`5`
              (`SkeletalMeshComponent.SetSkeletalMeshAsset` _skm_shirt_10 "/Game/ZombieMegaBundle/Mesh_UE5/UE5_Skeleton/Cloth/Sleeveless_Tshirt/Fat/SKM_Fat_Sleeveless_Tshirt_UE5.SKM_Fat_Sleeveless_Tshirt_UE5"))))
        (:`1`
          ;;[1 1 1 0.5] T-Shirt
          (switch `int` (`KismetMathLibrary.RandomInteger` 11)
            (:`0`
              (`SkeletalMeshComponent.SetSkeletalMeshAsset` _skm_shirt "/Game/ZombieMegaBundle/Mesh_UE5/UE5_Skeleton/Cloth/Tshirt/Fat/SKM_Fat_Tshirt_Black_Logo_UE5.SKM_Fat_Tshirt_Black_Logo_UE5"))
            (:`1`
              (`SkeletalMeshComponent.SetSkeletalMeshAsset` _skm_shirt "/Game/ZombieMegaBundle/Mesh_UE5/UE5_Skeleton/Cloth/Tshirt/Fat/SKM_Fat_Tshirt_Black_UE5.SKM_Fat_Tshirt_Black_UE5"))
            (:`2`
              (`SkeletalMeshComponent.SetSkeletalMeshAsset` _skm_shirt "/Game/ZombieMegaBundle/Mesh_UE5/UE5_Skeleton/Cloth/Tshirt/Fat/SKM_Fat_Tshirt_Blood_UE5.SKM_Fat_Tshirt_Blood_UE5"))
            (:`3`
              (`SkeletalMeshComponent.SetSkeletalMeshAsset` _skm_shirt "/Game/ZombieMegaBundle/Mesh_UE5/UE5_Skeleton/Cloth/Tshirt/Fat/SKM_Fat_Tshirt_Blue_Blood_UE5.SKM_Fat_Tshirt_Blue_Blood_UE5"))
            (:`4`
              (`SkeletalMeshComponent.SetSkeletalMeshAsset` _skm_shirt "/Game/ZombieMegaBundle/Mesh_UE5/UE5_Skeleton/Cloth/Tshirt/Fat/SKM_Fat_Tshirt_Green_Blood_UE5.SKM_Fat_Tshirt_Green_Blood_UE5"))
            (:`5`
              (`SkeletalMeshComponent.SetSkeletalMeshAsset` _skm_shirt "/Game/ZombieMegaBundle/Mesh_UE5/UE5_Skeleton/Cloth/Tshirt/Fat/SKM_Fat_Tshirt_Green_UE5.SKM_Fat_Tshirt_Green_UE5"))
            (:`6`
              (`SkeletalMeshComponent.SetSkeletalMeshAsset` _skm_shirt "/Game/ZombieMegaBundle/Mesh_UE5/UE5_Skeleton/Cloth/Tshirt/Fat/SKM_Fat_Tshirt_Logo_UE5.SKM_Fat_Tshirt_Logo_UE5"))
            (:`7`
              (`SkeletalMeshComponent.SetSkeletalMeshAsset` _skm_shirt "/Game/ZombieMegaBundle/Mesh_UE5/UE5_Skeleton/Cloth/Tshirt/Fat/SKM_Fat_Tshirt_White_Blood_UE5.SKM_Fat_Tshirt_White_Blood_UE5"))
            (:`8`
              (`SkeletalMeshComponent.SetSkeletalMeshAsset` _skm_shirt "/Game/ZombieMegaBundle/Mesh_UE5/UE5_Skeleton/Cloth/Tshirt/Fat/SKM_Fat_Tshirt_Blue_UE5.SKM_Fat_Tshirt_Blue_UE5"))
            (:`9`
              (`SkeletalMeshComponent.SetSkeletalMeshAsset` _skm_shirt "/Game/ZombieMegaBundle/Mesh_UE5/UE5_Skeleton/Cloth/Tshirt/Fat/SKM_Fat_Tshirt_White_UE5.SKM_Fat_Tshirt_White_UE5"))
            (:`10`
              (`SkeletalMeshComponent.SetSkeletalMeshAsset` _skm_shirt "/Game/ZombieMegaBundle/Mesh_UE5/UE5_Skeleton/Cloth/Tshirt/Fat/SKM_Fat_Tshirt_Fat_Black_Blood_UE5.SKM_Fat_Tshirt_Fat_Black_Blood_UE5"))))
        (:`2`
          ;;[1 1 1 0.5] T-Shirt Damaged
          (switch `int` (`KismetMathLibrary.RandomInteger` 3)
            (:`0`
              (`SkeletalMeshComponent.SetSkeletalMeshAsset` _skm_shirt_7 "/Game/ZombieMegaBundle/Mesh_UE5/UE5_Skeleton/Cloth/Tshirt_Demaged/Fat/SKM_Fat_TShirt_Damage_Black_UE5.SKM_Fat_TShirt_Damage_Black_UE5"))
            (:`1`
              (`SkeletalMeshComponent.SetSkeletalMeshAsset` _skm_shirt_7 "/Game/ZombieMegaBundle/Mesh_UE5/UE5_Skeleton/Cloth/Tshirt_Demaged/Fat/SKM_Fat_TShirt_Damage_Red_UE5.SKM_Fat_TShirt_Damage_Red_UE5"))
            (:`2`
              (`SkeletalMeshComponent.SetSkeletalMeshAsset` _skm_shirt_7 "/Game/ZombieMegaBundle/Mesh_UE5/UE5_Skeleton/Cloth/Tshirt_Demaged/Fat/SKM_Fat_TShirt_Damage_UE5.SKM_Fat_TShirt_Damage_UE5"))
            (:`3`
              (`SkeletalMeshComponent.SetSkeletalMeshAsset` _skm_shirt_7 "/Game/ZombieMegaBundle/Mesh_UE5/UE5_Skeleton/Cloth/Tshirt_Demaged/Fat/SKM_Fat_TShirt_Damage_White_UE5.SKM_Fat_TShirt_Damage_White_UE5"))))))))

(fn `SetShoesSKM`
  (switch `int` (`KismetMathLibrary.RandomInteger` 4)
    (:`1`
      (`SkeletalMeshComponent.SetSkeletalMeshAsset` (`self.SKM_Shoes`) "/Game/ZombieMegaBundle/Mesh_UE5/UE5_Skeleton/Boots/SKM_Classic_Boots_UE5.SKM_Classic_Boots_UE5"))
    (:`2`
      (`SkeletalMeshComponent.SetSkeletalMeshAsset` (`self.SKM_Shoes`) "/Game/ZombieMegaBundle/Mesh_UE5/UE5_Skeleton/Boots/SKM_Sneakers_Black_UE5.SKM_Sneakers_Black_UE5"))
    (:`3`
      (`SkeletalMeshComponent.SetSkeletalMeshAsset` (`self.SKM_Shoes`) "/Game/ZombieMegaBundle/Mesh_UE5/UE5_Skeleton/Boots/SKM_Sneakers_Red_UE5.SKM_Sneakers_Red_UE5"))
    (:`4`
      (`SkeletalMeshComponent.SetSkeletalMeshAsset` (`self.SKM_Shoes`) "/Game/ZombieMegaBundle/Mesh_UE5/UE5_Skeleton/Boots/SKM_Sneakers_UE5.SKM_Sneakers_UE5"))))

(fn `SetZombieAnimBP`
  (switch `EZombieType` (`self.ZombieType`)
    (:`Walker`
      (`SkeletalMeshComponent.SetAnimInstanceClass` (`self.Mesh`) "/Game/_Game/Characters/Zombies/ABP_Zombie_Walker.ABP_Zombie_Walker_C"))))

(fn `SetZombieBodySKM`
  (bind _mesh (`self.Mesh`))
  (bind _mesh_2 (`self.Mesh`))
  (bind _mesh_3 (`self.Mesh`))
  (bind _mesh_4 (`self.Mesh`))
  (bind _mesh_5 (`self.Mesh`))
  (bind _mesh_6 (`self.Mesh`))
  (bind _mesh_7 (`self.Mesh`))
  (bind _mesh_8 (`self.Mesh`))
  (switch `EZombieType` (`self.ZombieType`)
    (:`Walker`
      ;[1 1 1 0.5] Set Skinny (Walker) Body as Main Mesh
      (switch `int` (`KismetMathLibrary.RandomInteger` 3)
        (:`0`
          (set `SkeletalMeshComponent.SkeletalMeshAsset` "/Game/ZombieMegaBundle/Mesh_UE5/UE5_Skeleton/Body/SKM_Body_Skinny_UE5.SKM_Body_Skinny_UE5" _mesh_6)
          (`PrimitiveComponent.SetMaterial` _mesh_7 0 "/Game/ZombieMegaBundle/Materials/Body/M_Body_Skinny.M_Body_Skinny"))
        (:`1`
          (set `SkeletalMeshComponent.SkeletalMeshAsset` "/Game/ZombieMegaBundle/Mesh_UE5/UE5_Skeleton/Body/SKM_Body_Skinny_Blood_UE5.SKM_Body_Skinny_Blood_UE5" _mesh_6)
          (`PrimitiveComponent.SetMaterial` _mesh_7 0 "/Game/ZombieMegaBundle/Materials/Body/M_Body_Skinny_Blood.M_Body_Skinny_Blood"))
        (:`2`
          (set `SkeletalMeshComponent.SkeletalMeshAsset` "/Game/ZombieMegaBundle/Mesh_UE5/UE5_Skeleton/Body/SKM_Body_Skinny_ScarFace_Blood_UE5.SKM_Body_Skinny_ScarFace_Blood_UE5" _mesh_6)
          (`PrimitiveComponent.SetMaterial` _mesh_7 0 "/Game/ZombieMegaBundle/Materials/Body/M_Body_Skinny_ScarFase_Blood.M_Body_Skinny_ScarFase_Blood"))
        (:`3`
          (set `SkeletalMeshComponent.SkeletalMeshAsset` "/Game/ZombieMegaBundle/Mesh_UE5/UE5_Skeleton/Body/SKM_Body_Skinny_ScarFace_UE5.SKM_Body_Skinny_ScarFace_UE5" _mesh_6)
          (`PrimitiveComponent.SetMaterial` _mesh_7 0 "/Game/ZombieMegaBundle/Materials/Body/M_Body_Skinny_ScarFase.M_Body_Skinny_ScarFase"))))
    (:`Runner`
      ;[1 1 1 0.5] Set Normal (Runner) Body as Main Mesh
      (switch `int` (`KismetMathLibrary.RandomInteger` 2)
        (:`0`
          (set `SkeletalMeshComponent.SkeletalMeshAsset` "/Game/ZombieMegaBundle/Mesh_UE5/UE5_Skeleton/Body/SKM_Body_Normal_UE5.SKM_Body_Normal_UE5" _mesh_2)
          (`PrimitiveComponent.SetMaterial` _mesh_8 0 "/Game/ZombieMegaBundle/Materials/Body/M_Body_Normal.M_Body_Normal"))
        (:`1`
          (set `SkeletalMeshComponent.SkeletalMeshAsset` "/Game/ZombieMegaBundle/Mesh_UE5/UE5_Skeleton/Body/SKM_Body_Normal_Blood_UE5.SKM_Body_Normal_Blood_UE5" _mesh_2)
          (`PrimitiveComponent.SetMaterial` _mesh_8 0 "/Game/ZombieMegaBundle/Materials/Body/M_Body_Normal_Blood.M_Body_Normal_Blood"))
        (:`2`
          (set `SkeletalMeshComponent.SkeletalMeshAsset` "/Game/ZombieMegaBundle/Mesh_UE5/UE5_Skeleton/Body/SKM_Body_Afro_UE5.SKM_Body_Afro_UE5" _mesh_2)
          (`PrimitiveComponent.SetMaterial` _mesh_8 0 "/Game/ZombieMegaBundle/Materials/Body/M_Body_Normal_Afro.M_Body_Normal_Afro"))))
    (:`Tank`
      ;[1 1 1 0.5] Set Muscle (Tank) Body as Main Mesh
      (switch `int` (`KismetMathLibrary.RandomInteger` 2)
        (:`0`
          (set `SkeletalMeshComponent.SkeletalMeshAsset` "/Game/ZombieMegaBundle/Mesh_UE5/UE5_Skeleton/Body/SKM_Body_Muscle_UE5.SKM_Body_Muscle_UE5" _mesh_5)
          (`PrimitiveComponent.SetMaterial` _mesh 0 "/Game/ZombieMegaBundle/Materials/Body/M_Body_Muscle.M_Body_Muscle"))
        (:`1`
          (set `SkeletalMeshComponent.SkeletalMeshAsset` "/Game/ZombieMegaBundle/Mesh_UE5/UE5_Skeleton/Body/SKM_Body_Muscle_Blood_UE5.SKM_Body_Muscle_Blood_UE5" _mesh_5)
          (`PrimitiveComponent.SetMaterial` _mesh 0 "/Game/ZombieMegaBundle/Materials/Body/M_Body_Muscle_Blood.M_Body_Muscle_Blood"))
        (:`2`
          (set `SkeletalMeshComponent.SkeletalMeshAsset` "/Game/ZombieMegaBundle/Mesh_UE5/UE5_Skeleton/Body/SKM_Body_Muscle_Afro_UE5.SKM_Body_Muscle_Afro_UE5" _mesh_5)
          (`PrimitiveComponent.SetMaterial` _mesh 0 "/Game/ZombieMegaBundle/Materials/Body/M_Body_Muscle_Afro.M_Body_Muscle_Afro"))))
    (:`Bloater`
      ;[1 1 1 0.5] Set Fat (Bloater) Body as Main Mesh
      (switch `int` (`KismetMathLibrary.RandomInteger` 2)
        (:`0`
          (set `SkeletalMeshComponent.SkeletalMeshAsset` "/Game/ZombieMegaBundle/Mesh_UE5/UE5_Skeleton/Body/SKM_Body_Fat_UE5.SKM_Body_Fat_UE5" _mesh_4)
          (`PrimitiveComponent.SetMaterial` _mesh_3 0 "/Game/ZombieMegaBundle/Materials/Body/M_Body_Fat.M_Body_Fat"))
        (:`1`
          (set `SkeletalMeshComponent.SkeletalMeshAsset` "/Game/ZombieMegaBundle/Mesh_UE5/UE5_Skeleton/Body/SKM_Body_Fat_Blood_UE5.SKM_Body_Fat_Blood_UE5" _mesh_4)
          (`PrimitiveComponent.SetMaterial` _mesh_3 0 "/Game/ZombieMegaBundle/Materials/Body/M_Body_Fat_Blood.M_Body_Fat_Blood"))
        (:`2`
          (set `SkeletalMeshComponent.SkeletalMeshAsset` "/Game/ZombieMegaBundle/Mesh_UE5/UE5_Skeleton/Body/SKM_Body_Fat_Afro_UE5.SKM_Body_Fat_Afro_UE5" _mesh_4)
          (`PrimitiveComponent.SetMaterial` _mesh_3 0 "/Game/ZombieMegaBundle/Materials/Body/M_Body_Fat_Afro.M_Body_Fat_Afro"))))))

(fn `UserConstructionScript`
  (`self.BuildZombie`))