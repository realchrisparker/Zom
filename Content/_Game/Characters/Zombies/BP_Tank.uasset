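; BP_Tank is a muscular zombie character that randomizes its body and outfit in the Construction Script.
; BuildZombie picks a body mesh with matching material, then random shoes, pants, shirt and headwear or hair.
; Shoes and head can roll no new mesh, and the jacket step is an empty stub.
; All clothing meshes follow the body Mesh through Leader Pose so they animate as one.
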(fn `BuildZombie`
  (`|ExecutionSequence`
    (:`then_0`
      ;[1 1 1 0.5] Setup Body
      (`self.SetZombieBodySKM`))
    (:`then_1`
      ;[1 1 1 0.5] Set Shoes
      (`self.SetShoesSKM`)
      ;[1 1 1 0.5] Set Pants
      (`self.SetPantsSKM`)
      ;[1 1 1 0.5] Set Shirt
      (`self.SetShirtSKM`)
      ;[1 1 1 0.5] Set Jacket
      (`self.SetJacketSKM`)
      ;[1 1 1 0.5] Set Head
      (`self.SetHeadSKM`))
    (:`then_2`
      ;[1 1 1 0.5] Set leader pose to mesh so all sub SKM's act as one with the parent Mesh
      (`SkinnedMeshComponent.SetLeaderPoseComponent` (`self.SKM_Shoes`) (`self.Mesh`) false false)
      (`SkinnedMeshComponent.SetLeaderPoseComponent` (`self.SKM_Pants`) (`self.Mesh`) false false)
      (`SkinnedMeshComponent.SetLeaderPoseComponent` (`self.SKM_Shirt`) (`self.Mesh`) false false)
      (`SkinnedMeshComponent.SetLeaderPoseComponent` (`self.SKM_Jacket`) (`self.Mesh`) false false)
      (`SkinnedMeshComponent.SetLeaderPoseComponent` (`self.SKM_Head`) (`self.Mesh`) false false))))

(fn `SetHeadSKM`
  (bind _skm_head (`self.SKM_Head`))
  (bind _skm_head_2 (`self.SKM_Head`))
  (bind _skm_head_3 (`self.SKM_Head`))
  (switch `int` (`KismetMathLibrary.RandomInteger` 4)
    (:`1`
      ;[1 1 1 0.5] Ball Cap
      (switch `int` (`KismetMathLibrary.RandomInteger` 2)
        (:`0`
          (`SkeletalMeshComponent.SetSkeletalMeshAsset` _skm_head_3 "/Game/ZombieMegaBundle/Mesh_UE5/UE5_Skeleton/Head_Detals/SKM_Cap_Red_UE5.SKM_Cap_Red_UE5"))
        (:`1`
          (`SkeletalMeshComponent.SetSkeletalMeshAsset` _skm_head_3 "/Game/ZombieMegaBundle/Mesh_UE5/UE5_Skeleton/Head_Detals/SKM_Cap_UE5.SKM_Cap_UE5"))
        (:`2`
          (`SkeletalMeshComponent.SetSkeletalMeshAsset` _skm_head_3 "/Game/ZombieMegaBundle/Mesh_UE5/UE5_Skeleton/Head_Detals/SKM_Construction_Helmet_UE5.SKM_Construction_Helmet_UE5"))))
    (:`2`
      ;[1 1 1 0.5] Hair
      (switch `int` (`KismetMathLibrary.RandomInteger` 3)
        (:`0`
          (`SkeletalMeshComponent.SetSkeletalMeshAsset` _skm_head "/Game/ZombieMegaBundle/Mesh_UE5/UE5_Skeleton/Head_Detals/SKM_Hair_Back_Long_UE5.SKM_Hair_Back_Long_UE5"))
        (:`1`
          (`SkeletalMeshComponent.SetSkeletalMeshAsset` _skm_head "/Game/ZombieMegaBundle/Mesh_UE5/UE5_Skeleton/Head_Detals/SKM_Hair_Back_UE5.SKM_Hair_Back_UE5"))
        (:`2`
          (`SkeletalMeshComponent.SetSkeletalMeshAsset` _skm_head "/Game/ZombieMegaBundle/Mesh_UE5/UE5_Skeleton/Head_Detals/SKM_Hair_Short_UE5.SKM_Hair_Short_UE5"))
        (:`3`
          (`SkeletalMeshComponent.SetSkeletalMeshAsset` _skm_head "/Game/ZombieMegaBundle/Mesh_UE5/UE5_Skeleton/Head_Detals/SKM_Long_Hair_UE5.SKM_Long_Hair_UE5"))))
    (:`3`
      ;[1 1 1 0.5] Skull Cap
      (switch `int` (`KismetMathLibrary.RandomInteger` 2)
        (:`0`
          (`SkeletalMeshComponent.SetSkeletalMeshAsset` _skm_head_2 "/Game/ZombieMegaBundle/Mesh_UE5/UE5_Skeleton/Head_Detals/SKM_Warm_Hat_Black_UE5.SKM_Warm_Hat_Black_UE5"))
        (:`1`
          (`SkeletalMeshComponent.SetSkeletalMeshAsset` _skm_head_2 "/Game/ZombieMegaBundle/Mesh_UE5/UE5_Skeleton/Head_Detals/SKM_Warm_Hat_UE5.SKM_Warm_Hat_UE5"))))))

(fn `SetJacketSKM`)

(fn `SetPantsSKM`
  (bind _skm_pants (`self.SKM_Pants`))
  (switch `int` (`KismetMathLibrary.RandomInteger` 8)
    (:`0`
      (`SkeletalMeshComponent.SetSkeletalMeshAsset` _skm_pants "/Game/ZombieMegaBundle/Mesh_UE5/UE5_Skeleton/Pants/Muscle/SKM_Jeans_Long_Muscle_Blue_UE5.SKM_Jeans_Long_Muscle_Blue_UE5"))
    (:`1`
      (`SkeletalMeshComponent.SetSkeletalMeshAsset` _skm_pants "/Game/ZombieMegaBundle/Mesh_UE5/UE5_Skeleton/Pants/Muscle/SKM_Jeans_Long_Muscle_Gray_UE5.SKM_Jeans_Long_Muscle_Gray_UE5"))
    (:`2`
      (`SkeletalMeshComponent.SetSkeletalMeshAsset` _skm_pants "/Game/ZombieMegaBundle/Mesh_UE5/UE5_Skeleton/Pants/Muscle/SKM_Jeans_Long_Muscle_UE5.SKM_Jeans_Long_Muscle_UE5"))
    (:`3`
      (`SkeletalMeshComponent.SetSkeletalMeshAsset` _skm_pants "/Game/ZombieMegaBundle/Mesh_UE5/UE5_Skeleton/Pants/Muscle/SKM_Jeans_Shorts_Muscle_Blue_UE5.SKM_Jeans_Shorts_Muscle_Blue_UE5"))
    (:`4`
      (`SkeletalMeshComponent.SetSkeletalMeshAsset` _skm_pants "/Game/ZombieMegaBundle/Mesh_UE5/UE5_Skeleton/Pants/Muscle/SKM_Jeans_Shorts_Muscle_Gray_UE5.SKM_Jeans_Shorts_Muscle_Gray_UE5"))
    (:`5`
      (`SkeletalMeshComponent.SetSkeletalMeshAsset` _skm_pants "/Game/ZombieMegaBundle/Mesh_UE5/UE5_Skeleton/Pants/Muscle/SKM_Jeans_Shorts_Muscle_UE5.SKM_Jeans_Shorts_Muscle_UE5"))
    (:`6`
      (`SkeletalMeshComponent.SetSkeletalMeshAsset` _skm_pants "/Game/ZombieMegaBundle/Mesh_UE5/UE5_Skeleton/Pants/Muscle/SKM_Pants_Short_Muscle_Brown_UE5.SKM_Pants_Short_Muscle_Brown_UE5"))
    (:`7`
      (`SkeletalMeshComponent.SetSkeletalMeshAsset` _skm_pants "/Game/ZombieMegaBundle/Mesh_UE5/UE5_Skeleton/Pants/Muscle/SKM_Pants_Short_Muscle_Gray_UE5.SKM_Pants_Short_Muscle_Gray_UE5"))
    (:`8`
      (`SkeletalMeshComponent.SetSkeletalMeshAsset` _skm_pants "/Game/ZombieMegaBundle/Mesh_UE5/UE5_Skeleton/Pants/Muscle/SKM_Pants_Short_Muscle_UE5.SKM_Pants_Short_Muscle_UE5"))))

(fn `SetShirtSKM`
  (bind _skm_shirt (`self.SKM_Shirt`))
  (bind _skm_shirt_2 (`self.SKM_Shirt`))
  (bind _skm_shirt_3 (`self.SKM_Shirt`))
  (switch `int` (`KismetMathLibrary.RandomInteger` 3)
    (:`0`
      ;[1 1 1 0.5] Sleeveless T-Shirt
      (switch `int` (`KismetMathLibrary.RandomInteger` 3)
        (:`0`
          (`SkeletalMeshComponent.SetSkeletalMeshAsset` _skm_shirt "/Game/ZombieMegaBundle/Mesh_UE5/UE5_Skeleton/Cloth/Sleeveless_Tshirt/Muscle/SKM_Muscle_Sleeveless_Tshirt_Blood_UE5.SKM_Muscle_Sleeveless_Tshirt_Blood_UE5"))
        (:`1`
          (`SkeletalMeshComponent.SetSkeletalMeshAsset` _skm_shirt "/Game/ZombieMegaBundle/Mesh_UE5/UE5_Skeleton/Cloth/Sleeveless_Tshirt/Muscle/SKM_Muscle_Sleeveless_Tshirt_UE5.SKM_Muscle_Sleeveless_Tshirt_UE5"))
        (:`2`
          (`SkeletalMeshComponent.SetSkeletalMeshAsset` _skm_shirt "/Game/ZombieMegaBundle/Mesh_UE5/UE5_Skeleton/Cloth/Sleeveless_Tshirt/Muscle/SKM_Muscle_Sleeveless_Tshirt_White_Blood_UE5.SKM_Muscle_Sleeveless_Tshirt_White_Blood_UE5"))
        (:`3`
          (`SkeletalMeshComponent.SetSkeletalMeshAsset` _skm_shirt "/Game/ZombieMegaBundle/Mesh_UE5/UE5_Skeleton/Cloth/Sleeveless_Tshirt/Muscle/SKM_Muscle_Sleeveless_Tshirt_White_UE5.SKM_Muscle_Sleeveless_Tshirt_White_UE5"))))
    (:`1`
      ;[1 1 1 0.5] T-Shirt
      (switch `int` (`KismetMathLibrary.RandomInteger` 11)
        (:`0`
          (`SkeletalMeshComponent.SetSkeletalMeshAsset` _skm_shirt_2 "/Game/ZombieMegaBundle/Mesh_UE5/UE5_Skeleton/Cloth/Tshirt/Muscle/SKM_Muscle_Tsirt_Black_Blood_UE5.SKM_Muscle_Tsirt_Black_Blood_UE5"))
        (:`1`
          (`SkeletalMeshComponent.SetSkeletalMeshAsset` _skm_shirt_2 "/Game/ZombieMegaBundle/Mesh_UE5/UE5_Skeleton/Cloth/Tshirt/Muscle/SKM_Muscle_Tsirt_Black_UE5.SKM_Muscle_Tsirt_Black_UE5"))
        (:`2`
          (`SkeletalMeshComponent.SetSkeletalMeshAsset` _skm_shirt_2 "/Game/ZombieMegaBundle/Mesh_UE5/UE5_Skeleton/Cloth/Tshirt/Muscle/SKM_Muscle_Tsirt_Blood_UE5.SKM_Muscle_Tsirt_Blood_UE5"))
        (:`3`
          (`SkeletalMeshComponent.SetSkeletalMeshAsset` _skm_shirt_2 "/Game/ZombieMegaBundle/Mesh_UE5/UE5_Skeleton/Cloth/Tshirt/Muscle/SKM_Muscle_Tsirt_Blue_Blood_UE5.SKM_Muscle_Tsirt_Blue_Blood_UE5"))
        (:`4`
          (`SkeletalMeshComponent.SetSkeletalMeshAsset` _skm_shirt_2 "/Game/ZombieMegaBundle/Mesh_UE5/UE5_Skeleton/Cloth/Tshirt/Muscle/SKM_Muscle_Tsirt_Green_UE5.SKM_Muscle_Tsirt_Green_UE5"))
        (:`5`
          (`SkeletalMeshComponent.SetSkeletalMeshAsset` _skm_shirt_2 "/Game/ZombieMegaBundle/Mesh_UE5/UE5_Skeleton/Cloth/Tshirt/Muscle/SKM_Muscle_Tsirt_Logo_Black_UE5.SKM_Muscle_Tsirt_Logo_Black_UE5"))
        (:`6`
          (`SkeletalMeshComponent.SetSkeletalMeshAsset` _skm_shirt_2 "/Game/ZombieMegaBundle/Mesh_UE5/UE5_Skeleton/Cloth/Tshirt/Muscle/SKM_Muscle_Tsirt_Logo_UE5.SKM_Muscle_Tsirt_Logo_UE5"))
        (:`7`
          (`SkeletalMeshComponent.SetSkeletalMeshAsset` _skm_shirt_2 "/Game/ZombieMegaBundle/Mesh_UE5/UE5_Skeleton/Cloth/Tshirt/Muscle/SKM_Muscle_Tsirt_White_Blood_UE5.SKM_Muscle_Tsirt_White_Blood_UE5"))
        (:`8`
          (`SkeletalMeshComponent.SetSkeletalMeshAsset` _skm_shirt_2 "/Game/ZombieMegaBundle/Mesh_UE5/UE5_Skeleton/Cloth/Tshirt/Muscle/SKM_Muscle_Tsirt_Blue_UE5.SKM_Muscle_Tsirt_Blue_UE5"))
        (:`9`
          (`SkeletalMeshComponent.SetSkeletalMeshAsset` _skm_shirt_2 "/Game/ZombieMegaBundle/Mesh_UE5/UE5_Skeleton/Cloth/Tshirt/Muscle/SKM_Muscle_Tsirt_White_UE5.SKM_Muscle_Tsirt_White_UE5"))
        (:`10`
          (`SkeletalMeshComponent.SetSkeletalMeshAsset` _skm_shirt_2 "/Game/ZombieMegaBundle/Mesh_UE5/UE5_Skeleton/Cloth/Tshirt/Muscle/SKM_Muscle_Tsirt_Green_Blood_UE5.SKM_Muscle_Tsirt_Green_Blood_UE5"))))
    (:`2`
      ;[1 1 1 0.5] T-Shirt Damaged
      (switch `int` (`KismetMathLibrary.RandomInteger` 3)
        (:`0`
          (`SkeletalMeshComponent.SetSkeletalMeshAsset` _skm_shirt_3 "/Game/ZombieMegaBundle/Mesh_UE5/UE5_Skeleton/Cloth/Tshirt_Demaged/Muscle/SKM_Muscle_TShirt_Demaged_Black_UE5.SKM_Muscle_TShirt_Demaged_Black_UE5"))
        (:`1`
          (`SkeletalMeshComponent.SetSkeletalMeshAsset` _skm_shirt_3 "/Game/ZombieMegaBundle/Mesh_UE5/UE5_Skeleton/Cloth/Tshirt_Demaged/Muscle/SKM_Muscle_TShirt_Demaged_Red_UE5.SKM_Muscle_TShirt_Demaged_Red_UE5"))
        (:`2`
          (`SkeletalMeshComponent.SetSkeletalMeshAsset` _skm_shirt_3 "/Game/ZombieMegaBundle/Mesh_UE5/UE5_Skeleton/Cloth/Tshirt_Demaged/Muscle/SKM_Muscle_TShirt_Demaged_UE5.SKM_Muscle_TShirt_Demaged_UE5"))
        (:`3`
          (`SkeletalMeshComponent.SetSkeletalMeshAsset` _skm_shirt_3 "/Game/ZombieMegaBundle/Mesh_UE5/UE5_Skeleton/Cloth/Tshirt_Demaged/Muscle/SKM_Muscle_TShirt_Demaged_White_UE5.SKM_Muscle_TShirt_Demaged_White_UE5"))))))

(fn `SetShoesSKM`
  (switch `int` (`KismetMathLibrary.RandomInteger` 4)
    (:`1`
      (`SkeletalMeshComponent.SetSkeletalMeshAsset` (`self.SKM_Shoes`) "/Game/ZombieMegaBundle/Mesh_UE5/UE5_Skeleton/Boots/SKM_Classic_Boots_UE5.SKM_Classic_Boots_UE5"))
    (:`2`
      (`SkeletalMeshComponent.SetSkeletalMeshAsset` (`self.SKM_Shoes`) "/Game/ZombieMegaBundle/Mesh_UE5/UE5_Skeleton/Boots/SKM_Sneakers_Black_UE5.SKM_Sneakers_Black_UE5"))
    (:`3`
      (`SkeletalMeshComponent.SetSkeletalMeshAsset` (`self.SKM_Shoes`) "/Game/ZombieMegaBundle/Mesh_UE5/UE5_Skeleton/Boots/SKM_Sneakers_Red_UE5.SKM_Sneakers_Red_UE5"))
    (:`4`
      (`SkeletalMeshComponent.SetSkeletalMeshAsset` (`self.SKM_Shoes`) "/Game/ZombieMegaBundle/Mesh_UE5/UE5_Skeleton/Boots/SKM_Sneakers_UE5.SKM_Sneakers_UE5"))))

(fn `SetZombieBodySKM`
  (bind _mesh (`self.Mesh`))
  (bind _mesh_2 (`self.Mesh`))
  (switch `int` (`KismetMathLibrary.RandomInteger` 2)
    (:`0`
      (set `SkeletalMeshComponent.SkeletalMeshAsset` "/Game/ZombieMegaBundle/Mesh_UE5/UE5_Skeleton/Body/SKM_Body_Muscle_UE5.SKM_Body_Muscle_UE5" _mesh_2)
      (`PrimitiveComponent.SetMaterial` _mesh 0 "/Game/ZombieMegaBundle/Materials/Body/M_Body_Muscle.M_Body_Muscle"))
    (:`1`
      (set `SkeletalMeshComponent.SkeletalMeshAsset` "/Game/ZombieMegaBundle/Mesh_UE5/UE5_Skeleton/Body/SKM_Body_Muscle_Blood_UE5.SKM_Body_Muscle_Blood_UE5" _mesh_2)
      (`PrimitiveComponent.SetMaterial` _mesh 0 "/Game/ZombieMegaBundle/Materials/Body/M_Body_Muscle_Blood.M_Body_Muscle_Blood"))
    (:`2`
      (set `SkeletalMeshComponent.SkeletalMeshAsset` "/Game/ZombieMegaBundle/Mesh_UE5/UE5_Skeleton/Body/SKM_Body_Muscle_Afro_UE5.SKM_Body_Muscle_Afro_UE5" _mesh_2)
      (`PrimitiveComponent.SetMaterial` _mesh 0 "/Game/ZombieMegaBundle/Materials/Body/M_Body_Muscle_Afro.M_Body_Muscle_Afro"))))

(fn `UserConstructionScript`
  (`self.BuildZombie`))