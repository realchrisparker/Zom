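; Walker zombie Blueprint that assembles a randomized look in its Construction Script.
; BuildZombie picks a body mesh with matching material, then shoes, pants, shirt, jacket and headwear or hair through random switches, some nested by style.
; Leader Pose makes every clothing mesh follow the body's animation.
; Some rolls leave a slot unchanged, and several last cases are unreachable because RandomInteger excludes its max.
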(fn `BuildZombie`
  (`|ExecutionSequence`
    (:`then_0`
      ;[1 1 1 0.5] Setup Body
      (`self.SetZombieBodySKM`))
    (:`then_1`
      ;[1 1 1 0.5] Set Shoes
      (`self.SetShoesSKM`)
      ;[1 1 1 0.5] Set Pants
      (`self.SetPantsSKM`)
      ;[1 1 1 0.5] Set Shirt
      (`self.SetShirtSKM`)
      ;[1 1 1 0.5] Set Jacket
      (`self.SetJacketSKM`)
      ;[1 1 1 0.5] Set Head
      (`self.SetHeadSKM`))
    (:`then_2`
      ;[1 1 1 0.5] Set leader pose to mesh so all sub SKM's act as one with the parent Mesh
      (`SkinnedMeshComponent.SetLeaderPoseComponent` (`self.SKM_Shoes`) (`self.Mesh`) false false)
      (`SkinnedMeshComponent.SetLeaderPoseComponent` (`self.SKM_Pants`) (`self.Mesh`) false false)
      (`SkinnedMeshComponent.SetLeaderPoseComponent` (`self.SKM_Shirt`) (`self.Mesh`) false false)
      (`SkinnedMeshComponent.SetLeaderPoseComponent` (`self.SKM_Jacket`) (`self.Mesh`) false false)
      (`SkinnedMeshComponent.SetLeaderPoseComponent` (`self.SKM_Head`) (`self.Mesh`) false false))))

(fn `SetHeadSKM`
  (bind _skm_head (`self.SKM_Head`))
  (bind _skm_head_2 (`self.SKM_Head`))
  (bind _skm_head_3 (`self.SKM_Head`))
  (switch `int` (`KismetMathLibrary.RandomInteger` 4)
    (:`1`
      ;[1 1 1 0.5] Ball Cap
      (switch `int` (`KismetMathLibrary.RandomInteger` 2)
        (:`0`
          (`SkeletalMeshComponent.SetSkeletalMeshAsset` _skm_head_3 "/Game/ZombieMegaBundle/Mesh_UE5/UE5_Skeleton/Head_Detals/SKM_Cap_Red_UE5.SKM_Cap_Red_UE5"))
        (:`1`
          (`SkeletalMeshComponent.SetSkeletalMeshAsset` _skm_head_3 "/Game/ZombieMegaBundle/Mesh_UE5/UE5_Skeleton/Head_Detals/SKM_Cap_UE5.SKM_Cap_UE5"))
        (:`2`
          (`SkeletalMeshComponent.SetSkeletalMeshAsset` _skm_head_3 "/Game/ZombieMegaBundle/Mesh_UE5/UE5_Skeleton/Head_Detals/SKM_Construction_Helmet_UE5.SKM_Construction_Helmet_UE5"))))
    (:`2`
      ;[1 1 1 0.5] Hair
      (switch `int` (`KismetMathLibrary.RandomInteger` 3)
        (:`0`
          (`SkeletalMeshComponent.SetSkeletalMeshAsset` _skm_head "/Game/ZombieMegaBundle/Mesh_UE5/UE5_Skeleton/Head_Detals/SKM_Hair_Back_Long_UE5.SKM_Hair_Back_Long_UE5"))
        (:`1`
          (`SkeletalMeshComponent.SetSkeletalMeshAsset` _skm_head "/Game/ZombieMegaBundle/Mesh_UE5/UE5_Skeleton/Head_Detals/SKM_Hair_Back_UE5.SKM_Hair_Back_UE5"))
        (:`2`
          (`SkeletalMeshComponent.SetSkeletalMeshAsset` _skm_head "/Game/ZombieMegaBundle/Mesh_UE5/UE5_Skeleton/Head_Detals/SKM_Hair_Short_UE5.SKM_Hair_Short_UE5"))
        (:`3`
          (`SkeletalMeshComponent.SetSkeletalMeshAsset` _skm_head "/Game/ZombieMegaBundle/Mesh_UE5/UE5_Skeleton/Head_Detals/SKM_Long_Hair_UE5.SKM_Long_Hair_UE5"))))
    (:`3`
      ;[1 1 1 0.5] Skull Cap
      (switch `int` (`KismetMathLibrary.RandomInteger` 2)
        (:`0`
          (`SkeletalMeshComponent.SetSkeletalMeshAsset` _skm_head_2 "/Game/ZombieMegaBundle/Mesh_UE5/UE5_Skeleton/Head_Detals/SKM_Warm_Hat_Black_UE5.SKM_Warm_Hat_Black_UE5"))
        (:`1`
          (`SkeletalMeshComponent.SetSkeletalMeshAsset` _skm_head_2 "/Game/ZombieMegaBundle/Mesh_UE5/UE5_Skeleton/Head_Detals/SKM_Warm_Hat_UE5.SKM_Warm_Hat_UE5"))))))

(fn `SetJacketSKM`
  (bind _skm_jacket (`self.SKM_Jacket`))
  (switch `int` (`KismetMathLibrary.RandomInteger` 6)
    (:`0`
      (`SkeletalMeshComponent.SetSkeletalMeshAsset` _skm_jacket "/Game/ZombieMegaBundle/Mesh_UE5/UE5_Skeleton/Cloth_Top/SKM_Jaket_Dark_UE5.SKM_Jaket_Dark_UE5"))
    (:`1`
      (`SkeletalMeshComponent.SetSkeletalMeshAsset` _skm_jacket "/Game/ZombieMegaBundle/Mesh_UE5/UE5_Skeleton/Cloth_Top/SKM_Jaket_Jeans_Blue_UE5.SKM_Jaket_Jeans_Blue_UE5"))
    (:`2`
      (`SkeletalMeshComponent.SetSkeletalMeshAsset` _skm_jacket "/Game/ZombieMegaBundle/Mesh_UE5/UE5_Skeleton/Cloth_Top/SKM_Jaket_Jeans_Gray_UE5.SKM_Jaket_Jeans_Gray_UE5"))
    (:`3`
      (`SkeletalMeshComponent.SetSkeletalMeshAsset` _skm_jacket "/Game/ZombieMegaBundle/Mesh_UE5/UE5_Skeleton/Cloth_Top/SKM_Jaket_Jeans_Red_UE5.SKM_Jaket_Jeans_Red_UE5"))
    (:`4`
      (`SkeletalMeshComponent.SetSkeletalMeshAsset` _skm_jacket "/Game/ZombieMegaBundle/Mesh_UE5/UE5_Skeleton/Cloth_Top/SKM_Jaket_Jeans_UE5.SKM_Jaket_Jeans_UE5"))
    (:`5`
      (`SkeletalMeshComponent.SetSkeletalMeshAsset` _skm_jacket "/Game/ZombieMegaBundle/Mesh_UE5/UE5_Skeleton/Cloth_Top/SKM_Jaket_UE5.SKM_Jaket_UE5"))))

(fn `SetPantsSKM`
  (bind _skm_pants (`self.SKM_Pants`))
  (switch `int` (`KismetMathLibrary.RandomInteger` 16)
    (:`0`
      (`SkeletalMeshComponent.SetSkeletalMeshAsset` _skm_pants "/Game/ZombieMegaBundle/Mesh_UE5/UE5_Skeleton/Pants/SKM_Jeans_Half_Blue_UE5.SKM_Jeans_Half_Blue_UE5"))
    (:`1`
      (`SkeletalMeshComponent.SetSkeletalMeshAsset` _skm_pants "/Game/ZombieMegaBundle/Mesh_UE5/UE5_Skeleton/Pants/SKM_Jeans_Half_Gray_UE5.SKM_Jeans_Half_Gray_UE5"))
    (:`2`
      (`SkeletalMeshComponent.SetSkeletalMeshAsset` _skm_pants "/Game/ZombieMegaBundle/Mesh_UE5/UE5_Skeleton/Pants/SKM_Jeans_Half_UE5.SKM_Jeans_Half_UE5"))
    (:`3`
      (`SkeletalMeshComponent.SetSkeletalMeshAsset` _skm_pants "/Game/ZombieMegaBundle/Mesh_UE5/UE5_Skeleton/Pants/SKM_Jeans_Long_Blue_UE5.SKM_Jeans_Long_Blue_UE5"))
    (:`4`
      (`SkeletalMeshComponent.SetSkeletalMeshAsset` _skm_pants "/Game/ZombieMegaBundle/Mesh_UE5/UE5_Skeleton/Pants/SKM_Jeans_Long_Gray_UE5.SKM_Jeans_Long_Gray_UE5"))
    (:`5`
      (`SkeletalMeshComponent.SetSkeletalMeshAsset` _skm_pants "/Game/ZombieMegaBundle/Mesh_UE5/UE5_Skeleton/Pants/SKM_Jeans_Long_UE5.SKM_Jeans_Long_UE5"))
    (:`6`
      (`SkeletalMeshComponent.SetSkeletalMeshAsset` _skm_pants "/Game/ZombieMegaBundle/Mesh_UE5/UE5_Skeleton/Pants/SKM_Jeans_Shorts_Blue_UE5.SKM_Jeans_Shorts_Blue_UE5"))
    (:`7`
      (`SkeletalMeshComponent.SetSkeletalMeshAsset` _skm_pants "/Game/ZombieMegaBundle/Mesh_UE5/UE5_Skeleton/Pants/SKM_Jeans_Shorts_Gray_UE5.SKM_Jeans_Shorts_Gray_UE5"))
    (:`8`
      (`SkeletalMeshComponent.SetSkeletalMeshAsset` _skm_pants "/Game/ZombieMegaBundle/Mesh_UE5/UE5_Skeleton/Pants/SKM_Jeans_Shorts_UE5.SKM_Jeans_Shorts_UE5"))
    (:`9`
      (`SkeletalMeshComponent.SetSkeletalMeshAsset` _skm_pants "/Game/ZombieMegaBundle/Mesh_UE5/UE5_Skeleton/Pants/SKM_Pants_Half_Brown_UE5.SKM_Pants_Half_Brown_UE5"))
    (:`10`
      (`SkeletalMeshComponent.SetSkeletalMeshAsset` _skm_pants "/Game/ZombieMegaBundle/Mesh_UE5/UE5_Skeleton/Pants/SKM_Pants_Half_Gray_UE5.SKM_Pants_Half_Gray_UE5"))
    (:`11`
      (`SkeletalMeshComponent.SetSkeletalMeshAsset` _skm_pants "/Game/ZombieMegaBundle/Mesh_UE5/UE5_Skeleton/Pants/SKM_Pants_Half_UE5.SKM_Pants_Half_UE5"))
    (:`12`
      (`SkeletalMeshComponent.SetSkeletalMeshAsset` _skm_pants "/Game/ZombieMegaBundle/Mesh_UE5/UE5_Skeleton/Pants/SKM_Pants_Long_Brown_UE5.SKM_Pants_Long_Brown_UE5"))
    (:`13`
      (`SkeletalMeshComponent.SetSkeletalMeshAsset` _skm_pants "/Game/ZombieMegaBundle/Mesh_UE5/UE5_Skeleton/Pants/SKM_Pants_Long_Gray_UE5.SKM_Pants_Long_Gray_UE5"))
    (:`14`
      (`SkeletalMeshComponent.SetSkeletalMeshAsset` _skm_pants "/Game/ZombieMegaBundle/Mesh_UE5/UE5_Skeleton/Pants/SKM_Pants_Long_UE5.SKM_Pants_Long_UE5"))
    (:`15`
      (`SkeletalMeshComponent.SetSkeletalMeshAsset` _skm_pants "/Game/ZombieMegaBundle/Mesh_UE5/UE5_Skeleton/Pants/SKM_Pants_Short_Brown_UE5.SKM_Pants_Short_Brown_UE5"))
    (:`16`
      (`SkeletalMeshComponent.SetSkeletalMeshAsset` _skm_pants "/Game/ZombieMegaBundle/Mesh_UE5/UE5_Skeleton/Pants/SKM_Pants_Short_Gray_UE5.SKM_Pants_Short_Gray_UE5"))
    (:`17`
      (`SkeletalMeshComponent.SetSkeletalMeshAsset` _skm_pants "/Game/ZombieMegaBundle/Mesh_UE5/UE5_Skeleton/Pants/SKM_Pants_Short_UE5.SKM_Pants_Short_UE5"))))

(fn `SetShirtSKM`
  (bind _skm_shirt (`self.SKM_Shirt`))
  (bind _skm_shirt_2 (`self.SKM_Shirt`))
  (bind _skm_shirt_3 (`self.SKM_Shirt`))
  (bind _skm_shirt_4 (`self.SKM_Shirt`))
  (switch `int` (`KismetMathLibrary.RandomInteger` 4)
    (:`1`
      ;[1 1 1 0.5] Long Sleeve Shirt
      (switch `int` (`KismetMathLibrary.RandomInteger` 9)
        (:`0`
          (`SkeletalMeshComponent.SetSkeletalMeshAsset` _skm_shirt_2 "/Game/ZombieMegaBundle/Mesh_UE5/UE5_Skeleton/Cloth/Shirt/SKM_Shirt_Black_Blood_UE5.SKM_Shirt_Black_Blood_UE5"))
        (:`1`
          (`SkeletalMeshComponent.SetSkeletalMeshAsset` _skm_shirt_2 "/Game/ZombieMegaBundle/Mesh_UE5/UE5_Skeleton/Cloth/Shirt/SKM_Shirt_Black_UE5.SKM_Shirt_Black_UE5"))
        (:`2`
          (`SkeletalMeshComponent.SetSkeletalMeshAsset` _skm_shirt_2 "/Game/ZombieMegaBundle/Mesh_UE5/UE5_Skeleton/Cloth/Shirt/SKM_Shirt_Blood_UE5.SKM_Shirt_Blood_UE5"))
        (:`3`
          (`SkeletalMeshComponent.SetSkeletalMeshAsset` _skm_shirt_2 "/Game/ZombieMegaBundle/Mesh_UE5/UE5_Skeleton/Cloth/Shirt/SKM_Shirt_Blue_Blood_UE5.SKM_Shirt_Blue_Blood_UE5"))
        (:`4`
          (`SkeletalMeshComponent.SetSkeletalMeshAsset` _skm_shirt_2 "/Game/ZombieMegaBundle/Mesh_UE5/UE5_Skeleton/Cloth/Shirt/SKM_Shirt_Hawaii_Blue_UE5.SKM_Shirt_Hawaii_Blue_UE5"))
        (:`5`
          (`SkeletalMeshComponent.SetSkeletalMeshAsset` _skm_shirt_2 "/Game/ZombieMegaBundle/Mesh_UE5/UE5_Skeleton/Cloth/Shirt/SKM_Shirt_Hawaii_Red_UE5.SKM_Shirt_Hawaii_Red_UE5"))
        (:`6`
          (`SkeletalMeshComponent.SetSkeletalMeshAsset` _skm_shirt_2 "/Game/ZombieMegaBundle/Mesh_UE5/UE5_Skeleton/Cloth/Shirt/SKM_Shirt_UE5.SKM_Shirt_UE5"))
        (:`7`
          (`SkeletalMeshComponent.SetSkeletalMeshAsset` _skm_shirt_2 "/Game/ZombieMegaBundle/Mesh_UE5/UE5_Skeleton/Cloth/Shirt/SKM_Shirt_White_Blood_UE5.SKM_Shirt_White_Blood_UE5"))
        (:`8`
          (`SkeletalMeshComponent.SetSkeletalMeshAsset` _skm_shirt_2 "/Game/ZombieMegaBundle/Mesh_UE5/UE5_Skeleton/Cloth/Shirt/SKM_Shirt_Blue_UE5.SKM_Shirt_Blue_UE5"))
        (:`9`
          (`SkeletalMeshComponent.SetSkeletalMeshAsset` _skm_shirt_2 "/Game/ZombieMegaBundle/Mesh_UE5/UE5_Skeleton/Cloth/Shirt/SKM_Shirt_White_UE5.SKM_Shirt_White_UE5"))))
    (:`2`
      ;[1 1 1 0.5] Sleeveless T-Shirt
      (switch `int` (`KismetMathLibrary.RandomInteger` 3)
        (:`0`
          (`SkeletalMeshComponent.SetSkeletalMeshAsset` _skm_shirt_3 "/Game/ZombieMegaBundle/Mesh_UE5/UE5_Skeleton/Cloth/Sleeveless_Tshirt/SKM_Sleeveless_Tshirt_Blood_UE5.SKM_Sleeveless_Tshirt_Blood_UE5"))
        (:`1`
          (`SkeletalMeshComponent.SetSkeletalMeshAsset` _skm_shirt_3 "/Game/ZombieMegaBundle/Mesh_UE5/UE5_Skeleton/Cloth/Sleeveless_Tshirt/SKM_Sleeveless_Tshirt_UE5.SKM_Sleeveless_Tshirt_UE5"))
        (:`2`
          (`SkeletalMeshComponent.SetSkeletalMeshAsset` _skm_shirt_3 "/Game/ZombieMegaBundle/Mesh_UE5/UE5_Skeleton/Cloth/Sleeveless_Tshirt/SKM_Sleeveless_Tshirt_White_Blood_UE5.SKM_Sleeveless_Tshirt_White_Blood_UE5"))
        (:`3`
          (`SkeletalMeshComponent.SetSkeletalMeshAsset` _skm_shirt_3 "/Game/ZombieMegaBundle/Mesh_UE5/UE5_Skeleton/Cloth/Sleeveless_Tshirt/SKM_Sleeveless_Tshirt_White_UE5.SKM_Sleeveless_Tshirt_White_UE5"))))
    (:`3`
      ;[1 1 1 0.5] T-Shirt Damaged
      (switch `int` (`KismetMathLibrary.RandomInteger` 9)
        (:`0`
          (`SkeletalMeshComponent.SetSkeletalMeshAsset` _skm_shirt_4 "/Game/ZombieMegaBundle/Mesh_UE5/UE5_Skeleton/Cloth/Tshirt/SKM_Tshirt_Black_Blood_UE5.SKM_Tshirt_Black_Blood_UE5"))
        (:`1`
          (`SkeletalMeshComponent.SetSkeletalMeshAsset` _skm_shirt_4 "/Game/ZombieMegaBundle/Mesh_UE5/UE5_Skeleton/Cloth/Tshirt/SKM_Tshirt_Black_Logo_UE5.SKM_Tshirt_Black_Logo_UE5"))
        (:`2`
          (`SkeletalMeshComponent.SetSkeletalMeshAsset` _skm_shirt_4 "/Game/ZombieMegaBundle/Mesh_UE5/UE5_Skeleton/Cloth/Tshirt/SKM_Tshirt_Black_UE5.SKM_Tshirt_Black_UE5"))
        (:`3`
          (`SkeletalMeshComponent.SetSkeletalMeshAsset` _skm_shirt_4 "/Game/ZombieMegaBundle/Mesh_UE5/UE5_Skeleton/Cloth/Tshirt/SKM_Tshirt_Blood_UE5.SKM_Tshirt_Blood_UE5"))
        (:`4`
          (`SkeletalMeshComponent.SetSkeletalMeshAsset` _skm_shirt_4 "/Game/ZombieMegaBundle/Mesh_UE5/UE5_Skeleton/Cloth/Tshirt/SKM_Tshirt_Blue_UE5.SKM_Tshirt_Blue_UE5"))
        (:`5`
          (`SkeletalMeshComponent.SetSkeletalMeshAsset` _skm_shirt_4 "/Game/ZombieMegaBundle/Mesh_UE5/UE5_Skeleton/Cloth/Tshirt/SKM_Tshirt_Green_Blood_UE5.SKM_Tshirt_Green_Blood_UE5"))
        (:`6`
          (`SkeletalMeshComponent.SetSkeletalMeshAsset` _skm_shirt_4 "/Game/ZombieMegaBundle/Mesh_UE5/UE5_Skeleton/Cloth/Tshirt/SKM_Tshirt_Green_UE5.SKM_Tshirt_Green_UE5"))
        (:`7`
          (`SkeletalMeshComponent.SetSkeletalMeshAsset` _skm_shirt_4 "/Game/ZombieMegaBundle/Mesh_UE5/UE5_Skeleton/Cloth/Tshirt/SKM_Tshirt_UE5.SKM_Tshirt_UE5"))
        (:`8`
          (`SkeletalMeshComponent.SetSkeletalMeshAsset` _skm_shirt_4 "/Game/ZombieMegaBundle/Mesh_UE5/UE5_Skeleton/Cloth/Tshirt/SKM_Tshirt_Blue_Blood_UE5.SKM_Tshirt_Blue_Blood_UE5"))
        (:`9`
          (`SkeletalMeshComponent.SetSkeletalMeshAsset` _skm_shirt_4 "/Game/ZombieMegaBundle/Mesh_UE5/UE5_Skeleton/Cloth/Tshirt/SKM_Tshirt_White_Blood_UE5.SKM_Tshirt_White_Blood_UE5"))
        (:`10`
          (`SkeletalMeshComponent.SetSkeletalMeshAsset` _skm_shirt_4 "/Game/ZombieMegaBundle/Mesh_UE5/UE5_Skeleton/Cloth/Tshirt/SKM_Tshirt_White_UE5.SKM_Tshirt_White_UE5"))))
    (:`4`
      ;[1 1 1 0.5] T-Shirt
      (switch `int` (`KismetMathLibrary.RandomInteger` 3)
        (:`0`
          (`SkeletalMeshComponent.SetSkeletalMeshAsset` _skm_shirt "/Game/ZombieMegaBundle/Mesh_UE5/UE5_Skeleton/Cloth/Tshirt_Demaged/SKM_TShirt_Demaged_Black_UE5.SKM_TShirt_Demaged_Black_UE5"))
        (:`1`
          (`SkeletalMeshComponent.SetSkeletalMeshAsset` _skm_shirt "/Game/ZombieMegaBundle/Mesh_UE5/UE5_Skeleton/Cloth/Tshirt_Demaged/SKM_TShirt_Demaged_Red_UE5.SKM_TShirt_Demaged_Red_UE5"))
        (:`2`
          (`SkeletalMeshComponent.SetSkeletalMeshAsset` _skm_shirt "/Game/ZombieMegaBundle/Mesh_UE5/UE5_Skeleton/Cloth/Tshirt_Demaged/SKM_TShirt_Demaged_UE5.SKM_TShirt_Demaged_UE5"))
        (:`3`
          (`SkeletalMeshComponent.SetSkeletalMeshAsset` _skm_shirt "/Game/ZombieMegaBundle/Mesh_UE5/UE5_Skeleton/Cloth/Tshirt_Demaged/SKM_TShirt_Demaged_White_UE5.SKM_TShirt_Demaged_White_UE5"))))))

(fn `SetShoesSKM`
  (switch `int` (`KismetMathLibrary.RandomInteger` 4)
    (:`1`
      (`SkeletalMeshComponent.SetSkeletalMeshAsset` (`self.SKM_Shoes`) "/Game/ZombieMegaBundle/Mesh_UE5/UE5_Skeleton/Boots/SKM_Classic_Boots_UE5.SKM_Classic_Boots_UE5"))
    (:`2`
      (`SkeletalMeshComponent.SetSkeletalMeshAsset` (`self.SKM_Shoes`) "/Game/ZombieMegaBundle/Mesh_UE5/UE5_Skeleton/Boots/SKM_Sneakers_Black_UE5.SKM_Sneakers_Black_UE5"))
    (:`3`
      (`SkeletalMeshComponent.SetSkeletalMeshAsset` (`self.SKM_Shoes`) "/Game/ZombieMegaBundle/Mesh_UE5/UE5_Skeleton/Boots/SKM_Sneakers_Red_UE5.SKM_Sneakers_Red_UE5"))
    (:`4`
      (`SkeletalMeshComponent.SetSkeletalMeshAsset` (`self.SKM_Shoes`) "/Game/ZombieMegaBundle/Mesh_UE5/UE5_Skeleton/Boots/SKM_Sneakers_UE5.SKM_Sneakers_UE5"))))

(fn `SetZombieBodySKM`
  (bind _mesh (`self.Mesh`))
  (bind _mesh_2 (`self.Mesh`))
  (switch `int` (`KismetMathLibrary.RandomInteger` 3)
    (:`0`
      (set `SkeletalMeshComponent.SkeletalMeshAsset` "/Game/ZombieMegaBundle/Mesh_UE5/UE5_Skeleton/Body/SKM_Body_Skinny_UE5.SKM_Body_Skinny_UE5" _mesh)
      (`PrimitiveComponent.SetMaterial` _mesh_2 0 "/Game/ZombieMegaBundle/Materials/Body/M_Body_Skinny.M_Body_Skinny"))
    (:`1`
      (set `SkeletalMeshComponent.SkeletalMeshAsset` "/Game/ZombieMegaBundle/Mesh_UE5/UE5_Skeleton/Body/SKM_Body_Skinny_Blood_UE5.SKM_Body_Skinny_Blood_UE5" _mesh)
      (`PrimitiveComponent.SetMaterial` _mesh_2 0 "/Game/ZombieMegaBundle/Materials/Body/M_Body_Skinny_Blood.M_Body_Skinny_Blood"))
    (:`2`
      (set `SkeletalMeshComponent.SkeletalMeshAsset` "/Game/ZombieMegaBundle/Mesh_UE5/UE5_Skeleton/Body/SKM_Body_Skinny_ScarFace_Blood_UE5.SKM_Body_Skinny_ScarFace_Blood_UE5" _mesh)
      (`PrimitiveComponent.SetMaterial` _mesh_2 0 "/Game/ZombieMegaBundle/Materials/Body/M_Body_Skinny_ScarFase_Blood.M_Body_Skinny_ScarFase_Blood"))
    (:`3`
      (set `SkeletalMeshComponent.SkeletalMeshAsset` "/Game/ZombieMegaBundle/Mesh_UE5/UE5_Skeleton/Body/SKM_Body_Skinny_ScarFace_UE5.SKM_Body_Skinny_ScarFace_UE5" _mesh)
      (`PrimitiveComponent.SetMaterial` _mesh_2 0 "/Game/ZombieMegaBundle/Materials/Body/M_Body_Skinny_ScarFase.M_Body_Skinny_ScarFase"))))

(fn `UserConstructionScript`
  (`self.BuildZombie`))