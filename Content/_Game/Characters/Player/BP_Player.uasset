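; Player character Blueprint that toggles between no combat and unarmed combat using the NumPad 1 key.
; CombatState resets to None in construction, and UpdateCombat runs on BeginPlay and after each toggle.
; UpdateCombat registers data tables and chooser classes with the combat core, defense and hit reaction components.
; Unarmed supplies attack, dodge, parry and hit reaction sets, while None passes empty table lists.
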(event `self.ReceiveBeginPlay`
  ;[1 1 1 0.5] Set up combat
  (`self.UpdateCombat`))

(event `Key|NumPadOne`
  (params (Key :type "Key Structure"))
  (:`Pressed`
    (if (`|EnumEquality` (`self.CombatState`))
      (set `self.CombatState` "Unarmed")
      (else
        (set `self.CombatState` "None")))
    ;[1 1 1 0.5] Set up combat
    (`self.UpdateCombat`)))

(fn `UpdateCombat`
  (`self.CombatCoreComponent`
    (:`then`
      (switch `ECombatState` (`self.CombatState`)
        (:`None`
          ;[1 1 1 0.5] (Combat Unarmed) Register attack chooser, combat tables, defense chooser, defense tab, hit reaction chooser, and hit reaction tables.
          (`MCS_CombatCoreComponent.RegisterAttackSetsFromTables` (`self.CombatCoreComponent`) (`|MakeArray`) null)
          (`MCS_CombatDefenseComponent.RegisterDefenseSetsFromTables` (`self.CombatDefenseComponent`) (`|MakeArray`) null)
          (`MCS_CombatHitReactionComponent.RegisterHitReactionSetsFromTables` (`self.CombatHitReactionComponent`) (`|MakeArray`) null))
        (:`Unarmed`
          ;[1 1 1 0.5] (Combat Unarmed) Register attack chooser, combat tables, defense chooser, defense tables, hit reaction chooser, and hit reaction tables.
          (`MCS_CombatCoreComponent.RegisterAttackSetsFromTables` (`self.CombatCoreComponent`) (`|MakeArray` "/Game/_Game/Characters/Player/Combat/Tables/MCS_Unarmed_Combat_LightAttacks.MCS_Unarmed_Combat_LightAttacks" "/Game/_Game/Characters/Player/Combat/Tables/MCS_Unarmed_Combat_HeavyAttacks.MCS_Unarmed_Combat_HeavyAttacks" :!type "DataTable Object Reference") "/Game/_Game/Characters/Player/Combat/Choosers/MCSAC_Player_Combat_Unarmed.MCSAC_Player_Combat_Unarmed_C")
          (`MCS_CombatDefenseComponent.RegisterDefenseSetsFromTables` (`self.CombatDefenseComponent`) (`|MakeArray` "/Game/_Game/Characters/Player/Combat/Tables/MCS_Unarmed_Combat_Dodges.MCS_Unarmed_Combat_Dodges" "/Game/_Game/Characters/Player/Combat/Tables/MCS_Unarmed_Combat_Parry.MCS_Unarmed_Combat_Parry" :!type "DataTable Object Reference") "/Game/_Game/Characters/Player/Combat/Choosers/MCSDC_Player_Combat_Unarmed.MCSDC_Player_Combat_Unarmed_C")
          (`MCS_CombatHitReactionComponent.RegisterHitReactionSetsFromTables` (`self.CombatHitReactionComponent`) (`|MakeArray` "/Game/_Game/Characters/Player/Combat/Tables/MCS_Unarmed_Combat_HitReactions.MCS_Unarmed_Combat_HitReactions" :!type "DataTable Object Reference") "/Game/_Game/Characters/Player/Combat/Choosers/MCSHR_Player_Combat_Unarmed.MCSHR_Player_Combat_Unarmed_C"))))
    (:`else`)))

(fn `UserConstructionScript`
  (set `self.CombatState` "None"))